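; Lobby player controller that sets up the lobby UI and handles adding clothing items to the shop checkout.
; BeginPlay runs high graphics console commands, caches the GI_Multix game instance, and shows the mobile lobby widget whatever the platform; the PC widget branch is disconnected.
; SetClothesID creates a checkout item widget in each top-level shop widget found, updating its total price and new-item list.
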(event `self.ReceiveBeginPlay`
  (for _array_element (`self.GraphicSettingsArrayHigh`)
    (`KismetSystemLibrary.ExecuteConsoleCommand` _array_element self))
  (`self.FCasts`)
  (switch `string` (`/MultixOnline/Blueprints/GI_Multix.GI_PlatformName` (`self.As GI Multix`))
    (:`Default`
      _)
    (:`Windows`
      _)
    (:`Android`
      _))
  ;[1 1 1] WBP_LobbyMain - Android
  (bind _returnvalue (`|CreateWidget` "/Game/_Mobile/Gamefolder/Rian/Widgets/LobbyMain/WBP_LobbyMain_Mobile.WBP_LobbyMain_Mobile_C" self))
  (bind _output_get (set `self.As WBP LobbyMain_Mobile` _returnvalue))
  (`UserWidget.AddToViewport` _output_get 0)
  (`WidgetBlueprintLibrary.SetInputMode_GameAndUIEx` self null "DoNotLock" false))

(event `SetClothesID`
  (params (ClothesID :type String) (Name :type Text) (Price :type Integer) (Image :type "Texture2D Object Reference") (isEnable :type Boolean))
  (bind _returnvalue (`|CreateWidget` "/Game/Gamefolder/Rian/Widgets/Lobby_Shop/WBP_Shop_CheckoutItems.WBP_Shop_CheckoutItems_C" null Name Price Image ClothesID isEnable))
  (bind _foundwidgets (`WidgetBlueprintLibrary.GetAllWidgetsOfClass` "/Game/Gamefolder/Rian/Widgets/Lobby_Shop/WBP_Shop.WBP_Shop_C"))
  (for _array_element _foundwidgets
    (`Widget.SetVisibility` (`/Game/Gamefolder/Rian/Widgets/Lobby_Shop/WBP_Shop.CheckoutWrapper` _array_element) "Visible")
    (`PanelWidget.AddChild` (`/Game/Gamefolder/Rian/Widgets/Lobby_Shop/WBP_Shop.CheckoutItems` _array_element) _returnvalue)
    (bind _output_get (set `/Game/Gamefolder/Rian/Widgets/Lobby_Shop/WBP_Shop.TotalPriceCheckout` (+ (`/Game/Gamefolder/Rian/Widgets/Lobby_Shop/WBP_Shop.TotalPriceCheckout` _array_element) Price) _array_element))
    (`TextBlock.SetText` (`/Game/Gamefolder/Rian/Widgets/Lobby_Shop/WBP_Shop.TotalPriceObject` _array_element) (`KismetTextLibrary.Conv_IntToText` _output_get))
    (`KismetArrayLibrary.Array_Add` (`/Game/Gamefolder/Rian/Widgets/Lobby_Shop/WBP_Shop.newItem` _array_element) ClothesID)))

(fn `FCasts`
  (`self.As GI Multix`
    (:`then`
      _)
    (:`else`
      (bind _asgi_multix (cast `/MultixOnline/Blueprints/GI_Multix` (`GameplayStatics.GetGameInstance`)))
      (set `self.As GI Multix` _asgi_multix)))
  (return))

(fn `UserConstructionScript`)