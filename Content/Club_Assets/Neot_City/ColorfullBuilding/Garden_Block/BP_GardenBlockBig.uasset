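; BP_GardenBlockBig is a garden block actor for the city that shows itself only while the player is nearby, acting as simple distance-based visibility culling.
; Every Tick it measures the distance to the BP_PlayerCharacter against a fixed threshold, unhiding within range and hiding beyond it.
; Two cross-resetting DoOnce nodes ensure each visibility change runs only once per threshold crossing.
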(event `self.ReceiveTick`
  (params (DeltaSeconds :type "Float (single-precision)"))
  (if (<= (`self.GetDistanceTo` (cast `/Game/Blueprints/Character/BP_PlayerCharacter` (`GameplayStatics.GetPlayerCharacter` 0) :!pure true)) 1500.0)
    (`|ExecutionSequence`
      (:`then_0`
        (`/Engine/EditorBlueprintResources/StandardMacros.DoOnce` false :!label _label
          (:`Completed`
            (`self.SetActorHiddenInGame` false))))
      (:`then_1`
        (goto _label_2 :!via `Reset`)))
    (else
      (`|ExecutionSequence`
        (:`then_0`
          (`/Engine/EditorBlueprintResources/StandardMacros.DoOnce` false :!label _label_2
            (:`Completed`
              (`self.SetActorHiddenInGame` true))))
        (:`then_1`
          (goto _label :!via `Reset`))))))

(fn `UserConstructionScript`)