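; Game State that acts as the hub for player registration, roster sync, logout, friend requests, private chat (WIP) and private voice calls.
; It keeps the roster in BP_GameInstance's PlayerDataArray, cached at BeginPlay, and relays changes and requests to the relevant BP_PlayerState.
; Roster, friend-request and logout events wait 0.1s so the cached GameInstance is ready.
; Chat and call interface events check the target is in the roster before forwarding.
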(event `self.ReceiveBeginPlay`
  ;[0 0 0 1 15] Notes: Please do not get the value from GameInstance here, u wont get anything because GameState works on Server even tho this is valid. If u want get the value from GameInstance in here, create RPC/OnRep function in GameState and call it from PlayerState or PlayerCharacter/PlayerController, example: Multicast_RetrievePlayerData
  (bind _asbp_game_instance (cast `/Game/Blueprints/Subsystem/BP_GameInstance` (`GameplayStatics.GetGameInstance`))
    (:`then`
      (set `self.As BP Game Instance` _asbp_game_instance))
    (:`CastFailed`
      (`KismetSystemLibrary.PrintString` "Game Instance Invalid"))))

(event `Server_RegisterPlayerState`
  (params (NewPlayerState :type "PlayerState Object Reference"))
  (bind _asbp_player_state (cast `/Game/Blueprints/PlayerState/BP_PlayerState` NewPlayerState))
  (`/Game/Blueprints/PlayerState/BP_PlayerState.Client_SetPlayerName` _asbp_player_state NewPlayerState))

(event `Multicast_RetrievePlayerData`
  (params (PlayerData :type "/Game/Blueprints/Structure/S_PlayerData Structure"))
  (`KismetSystemLibrary.Delay` 0.1) ; Server faster than BeginPlay, to reduce casting, we need Delay 0.1s
  (bind _as_bp_game_instance (`self.As BP Game Instance`)
    (:`then`
      (bind _playerdataarray (`/Game/Blueprints/Subsystem/BP_GameInstance.PlayerDataArray` _as_bp_game_instance))
      (if (not (`KismetArrayLibrary.Array_Contains` _playerdataarray PlayerData))
        (`KismetArrayLibrary.Array_Add` _playerdataarray PlayerData)
        (for _array_element _playerdataarray
          (bind _playerstate (break `/Game/Blueprints/Structure/S_PlayerData` _array_element))
          (`/Engine/EditorBlueprintResources/StandardMacros.IsValid` _playerstate
            (:`Is Valid`
              _)
            (:`Is Not Valid`
              (`KismetArrayLibrary.Array_RemoveItem` _playerdataarray _array_element)))
          (bind _asbp_player_state (cast `/Game/Blueprints/PlayerState/BP_PlayerState` _playerstate))
          (`/Game/Blueprints/PlayerState/BP_PlayerState.Client_RetrievePlayerData` _asbp_player_state _playerdataarray))))
    (:`else`)))

(event `Multicast_SendFriendsRequest`
  (params (ReceiverPlayer :type "/Game/Blueprints/Structure/S_PlayerData Structure") (SenderPlayer :type "/Game/Blueprints/Structure/S_PlayerData Structure"))
  (`KismetSystemLibrary.Delay` 0.1) ; Server faster than BeginPlay, to reduce casting, we need Delay 0.1s
  (bind _as_bp_game_instance (`self.As BP Game Instance`)
    (:`then`
      (if (`KismetArrayLibrary.Array_Contains` (`/Game/Blueprints/Subsystem/BP_GameInstance.PlayerDataArray` _as_bp_game_instance) ReceiverPlayer)
        (bind _asbp_player_state (cast `/Game/Blueprints/PlayerState/BP_PlayerState` (`.PlayerState_97_E5997660489A2A7EEEE909AD13D4D6C7` (break `/Game/Blueprints/Structure/S_PlayerData` ReceiverPlayer))))
        (`/Engine/EditorBlueprintResources/StandardMacros.IsValid` _asbp_player_state
          (:`Is Valid`
            (`/Game/Blueprints/PlayerState/BP_PlayerState.Client_SendFriendsRequest` _asbp_player_state ReceiverPlayer SenderPlayer)
            (`KismetSystemLibrary.PrintString` (`KismetStringLibrary.Concat_StrStr` "GameState || " "Sender: " (`KismetSystemLibrary.GetDisplayName` (`.PlayerState_97_E5997660489A2A7EEEE909AD13D4D6C7` (break `/Game/Blueprints/Structure/S_PlayerData` SenderPlayer))) " Receiver: " (`KismetSystemLibrary.GetDisplayName` (`.PlayerState_97_E5997660489A2A7EEEE909AD13D4D6C7` (break `/Game/Blueprints/Structure/S_PlayerData` ReceiverPlayer)))) true true (struct :`G` 0.66 :`B` 1.0 :`A` 1.0) 20.0)))))
    (:`else`)))

(event `Server_PlayerLogout`
  (params (PlayerState :type "PlayerState Object Reference"))
  (bind _playerlogout (`self.PlayerLogout`))
  (`KismetSystemLibrary.Delay` 0.1) ; Server faster than BeginPlay, to reduce casting, we need Delay 0.1s
  (bind _as_bp_game_instance (`self.As BP Game Instance`)
    (:`then`
      (bind _playerdataarray (`/Game/Blueprints/Subsystem/BP_GameInstance.PlayerDataArray` _as_bp_game_instance))
      (for _array_element _playerdataarray
        (bind _playerstate (break `/Game/Blueprints/Structure/S_PlayerData` _array_element))
        (if (== PlayerState _playerstate)
          (if (not (`KismetArrayLibrary.Array_Contains` _playerlogout _array_element))
            (`KismetArrayLibrary.Array_Add` _playerlogout _array_element))
          (`KismetArrayLibrary.Array_RemoveItem` _playerdataarray _array_element)
          (bind _asbp_player_state (cast `/Game/Blueprints/PlayerState/BP_PlayerState` _playerstate))
          (`/Game/Blueprints/PlayerState/BP_PlayerState.Client_RetrievePlayerData` _asbp_player_state _playerdataarray)
          (`/Game/Blueprints/PlayerState/BP_PlayerState.Client_PlayerLogout` _asbp_player_state (`self.PlayerLogout`)))))
    (:`else`)))

(event `/Game/Blueprints/Interface/BPI_InteractionInterface.FriendsRequestNotification`
  (params (ReceiverDataPlayer :type "/Game/Blueprints/Structure/S_PlayerData Structure"))
  (if (`KismetArrayLibrary.Array_Contains` (`/Game/Blueprints/Subsystem/BP_GameInstance.PlayerDataArray` (`self.As BP Game Instance`)) ReceiverDataPlayer)
    (`/Game/Blueprints/PlayerState/BP_PlayerState.Client_SendFriendsRequest` :`self` (cast `/Game/Blueprints/PlayerState/BP_PlayerState` (`.PlayerState_97_E5997660489A2A7EEEE909AD13D4D6C7` (break `/Game/Blueprints/Structure/S_PlayerData` ReceiverDataPlayer)) :!pure true) :`ReceiverPlayer` ReceiverDataPlayer)))

(event `/Game/Blueprints/Interface/BPI_InteractionInterface.BPIF Chat Send Message`
  (params (Rec_DataPlayer :type "/Game/Blueprints/Structure/S_PlayerData Structure"))
  (bind (_playerstate _playername) (break `/Game/Blueprints/Structure/S_PlayerData` Rec_DataPlayer))
  ;[1 0.9039 0] WIP: Replication for Privcate Chat
  ; Run on GameState Serverside
  ; Check
  ;;[1 1 1] Check if Playerdata yang dituju ada dalam array
  (if (`KismetArrayLibrary.Array_Contains` (`/Game/Blueprints/Subsystem/BP_GameInstance.PlayerDataArray` (`self.As BP Game Instance`)) Rec_DataPlayer)
    (`KismetSystemLibrary.PrintString` (`KismetStringLibrary.Concat_StrStr` "Yoyoy: " _playername))
    (`/Game/Blueprints/PlayerState/BP_PlayerState.OC_SendMessage` :`self` (cast `/Game/Blueprints/PlayerState/BP_PlayerState` _playerstate :!pure true) :`PlayerName` (`KismetStringLibrary.Concat_StrStr` "Burgerking: " _playername)) ; Send Message to PlayerState
  ))

(event `/Game/Blueprints/Interface/BPI_InteractionInterface.BPIF_PV0_ReceiveCallRequest`
  (params (`Sender PlayerData` :type "/Game/Blueprints/Structure/S_PlayerData Structure") (`Receiver PlayerData` :type "/Game/Blueprints/Structure/S_PlayerData Structure"))
  (bind (_playerstate _playername) (break `/Game/Blueprints/Structure/S_PlayerData` `Receiver PlayerData`))
  ;[1 1 1] Check if Playerdata yang dituju ada dalam array
  (if (`KismetArrayLibrary.Array_Contains` (`/Game/Blueprints/Subsystem/BP_GameInstance.PlayerDataArray` (`self.As BP Game Instance`)) `Receiver PlayerData`)
    (`KismetSystemLibrary.PrintString` (`KismetStringLibrary.Concat_StrStr` "In GameState: " _playername))
    (`/Game/Blueprints/PlayerState/BP_PlayerState.OC_ReceiveCallRequest` (cast `/Game/Blueprints/PlayerState/BP_PlayerState` _playerstate :!pure true) `Sender PlayerData` `Receiver PlayerData`) ; Send Voice Request to Receiver?
    (else
      (`KismetSystemLibrary.PrintString` "Array PlayerData cannot find specified user" true true (struct :`R` 1.0 :`B` 0.035615 :`A` 1.0) 5.0))))

(event `/Game/Blueprints/Interface/BPI_InteractionInterface.BPIF_PV1_ReceiverAcceptSenderConnect`
  (params (Sender :type "/Game/Blueprints/Structure/S_PlayerData Structure") (Receiver :type "/Game/Blueprints/Structure/S_PlayerData Structure"))
  (bind (_playerstate _playername) (break `/Game/Blueprints/Structure/S_PlayerData` Sender))
  ;[1 1 1] Check if Playerdata yang dituju ada dalam array
  (if (`KismetArrayLibrary.Array_Contains` (`/Game/Blueprints/Subsystem/BP_GameInstance.PlayerDataArray` (`self.As BP Game Instance`)) Receiver)
    (`KismetSystemLibrary.PrintString` (`KismetStringLibrary.Concat_StrStr` "In GameState: " _playername))
    (`/Game/Blueprints/PlayerState/BP_PlayerState.OC_ReceiverAcceptedPV_ConnectVoice` (cast `/Game/Blueprints/PlayerState/BP_PlayerState` _playerstate :!pure true) Sender Receiver)))

(fn `BPIF_GetInventoryArray`
  (returns (Inventory_Roses :type "Array of Integer") (Inventory_Guns :type "Array of Integer") (Inventory_AvatarItems :type "Array of Integer"))
  (return))

(fn `BPIF_GetPoints`
  (returns (mXRUN :type Integer) (XRUN :type Integer))
  (return 0 0))

(fn `UserConstructionScript`)