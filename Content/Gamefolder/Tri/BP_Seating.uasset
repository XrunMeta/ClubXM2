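; BP_Seating is a seat actor that characters can sit on while it is empty.
; Box overlap gives BP_Character its CanSit flag, seat transform and actor reference and shows SeatAnim and TextRender; end overlap clears the flag and hides both.
; ChangeSeatStatus flips IsEmptySeat only on authority.
; The WBP_SeatStatus label updates are disconnected and never run.
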(event `ChangeSeatStatus`
  (`/Engine/EditorBlueprintResources/ActorMacros.Switch Has Authority`
    (:`Authority`
      (`self.Toggle Seat`))))

(event `Toggle Seat`
  (if (`self.IsEmptySeat?`)
    (set `self.IsEmptySeat?` false)
    (else
      (set `self.IsEmptySeat?` true))))

(event `self.ReceiveBeginPlay`)

(event `self.Box.OnComponentBeginOverlap`
  (params (OverlappedComponent :type "PrimitiveComponent Object Reference") (OtherActor :type "Actor Object Reference") (OtherComp :type "PrimitiveComponent Object Reference") (OtherBodyIndex :type Integer) (bFromSweep :type Boolean) (SweepResult :type "HitResult Structure (by ref)"))
  (if (`self.IsEmptySeat?`)
    (bind _asbp_character (cast `/MultixOnline/Blueprints/BP_Character` OtherActor))
    (set `/MultixOnline/Blueprints/BP_Character.CanSit` true _asbp_character)
    (set `/MultixOnline/Blueprints/BP_Character.SeatRotation` (`SceneComponent.K2_GetComponentRotation` (`self.Arrow`)) _asbp_character)
    (set `/MultixOnline/Blueprints/BP_Character.Seat_Location` (`SceneComponent.K2_GetComponentLocation` (`self.Character_Seat_Position`)) _asbp_character)
    (set `/MultixOnline/Blueprints/BP_Character.SeatActor` self _asbp_character)
    (`SceneComponent.SetVisibility` (`self.SeatAnim`) true false)
    (`SceneComponent.SetVisibility` (`self.TextRender`) true false)))

(event `self.Box.OnComponentEndOverlap`
  (params (OverlappedComponent :type "PrimitiveComponent Object Reference") (OtherActor :type "Actor Object Reference") (OtherComp :type "PrimitiveComponent Object Reference") (OtherBodyIndex :type Integer))
  (bind _asbp_character (cast `/MultixOnline/Blueprints/BP_Character` OtherActor))
  (set `/MultixOnline/Blueprints/BP_Character.CanSit` false _asbp_character)
  (`SceneComponent.SetVisibility` (`self.SeatAnim`) false false)
  (`SceneComponent.SetVisibility` (`self.TextRender`) false false))

(fn `FCast`
  (bind _asgs_multix_gameplay (cast `/MultixOnline/Blueprints/GS_MultixGameplay` (`GameplayStatics.GetGameState`)))
  (set `self.As GS Multix Gameplay` _asgs_multix_gameplay))

(fn `UserConstructionScript`)