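; Lobby game mode Blueprint that currently holds only disconnected test and draft logic, with BeginPlay and PostLogin left empty.
; Unwired VaRest chains sketch a getMaintenance API status check and an OpenWeatherMap test request, whose response handlers print results.
; An unwired player-registration chain maps each BP_PlayerState to PlayerInfoSubsystem data, and a comment says PostLogin logic belongs in BP_GameplayGameMode.
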(event `RestCallback`
  (params (Request :type "VaRestRequestJSON Object Reference"))
  ;[1 1 1] Test, and it works!
  (bind _returnvalue (`VaRestJsonValue.AsObject` (`|GetArrayItem` (`VaRestJsonObject.GetArrayField` (`VaRestRequestJSON.GetResponseObject` Request) "weather"))))
  (`KismetSystemLibrary.PrintString` (`VaRestJsonObject.GetStringField` _returnvalue "description")))

(event `self.ReceiveBeginPlay`)

(event `OnRequestComplete_Event`
  (params (Request :type "VaRestRequestJSON Object Reference"))
  (bind _returnvalue (`VaRestJsonValue.AsObject` (`|GetArrayItem` (`VaRestJsonObject.GetArrayField` (`VaRestRequestJSON.GetResponseObject` Request) "data"))))
  (if (`KismetStringLibrary.EqualEqual_StrStr` (`VaRestJsonObject.GetStringField` _returnvalue "status") "1")
    (`KismetSystemLibrary.PrintString` "Client's invalid" true true (struct :`R` 1.0 :`B` 0.037924 :`A` 1.0))
    (else
      (`KismetSystemLibrary.PrintString` "Client's Valid" true true (struct :`R` 0.06965 :`G` 1.0 :`A` 1.0)))))

(event `self.K2_PostLogin`
  (params (NewPlayer :type "PlayerController Object Reference"))
  ;[0 0 0 1 15] The logic should applied in BP_GameplayGameMode
)

(fn `UserConstructionScript`)