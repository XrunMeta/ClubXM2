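; Base NPC character Blueprint that handles projectile hit reactions, death and a dialog widget that faces the player.
; A looping timer rotates the talk widget component toward the player camera.
; Projectile hits play a react montage, then either increment CurrentHit or, when MaxHit >= CurrentHit, play a death montage and destroy the actor after a delay.
; The equipped-check interface function always reports no weapon.
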(event `Face Dialog to Player`
  (params (Delay :type "Float (double-precision)" :default 0.1) (CWBP :type "WidgetComponent Object Reference"))
  ;[0 0 0] Set Rotation for Widget Comp to facing the player
  (`KismetSystemLibrary.K2_SetTimerDelegate` (delegate `FaceDialogToPlayer`) Delay true))

(event `FaceDialogToPlayer`
  (bind _cwbp_npctalk (`self.CWBP_NPCTalk`))
  ;[0 0 0] Set Rotation for Widget Comp to facing the player
  (`/Engine/EditorBlueprintResources/StandardMacros.IsValid` _cwbp_npctalk
    (:`Is Valid`
      (`SceneComponent.K2_SetWorldRotation` _cwbp_npctalk (`KismetMathLibrary.FindLookAtRotation` (`SceneComponent.K2_GetComponentLocation` _cwbp_npctalk) (`self.K2_GetActorLocation` (`GameplayStatics.GetPlayerCameraManager` 0))) false false))))

(event `self.ReceiveTick`
  (params (DeltaSeconds :type "Float (single-precision)")))

(event `Hit By Projectile`
  (`self.PlayAnimMontage` "/Game/Assets/Animation/Mon_Hit_React_1.Mon_Hit_React_1")
  (`KismetSystemLibrary.PrintString` "I'm Hit!")
  (if (>= (`self.Max Hit`) (`self.Current Hit`))
    (`self.PlayAnimMontage` "/Game/Fantasy_Pack/Animations/2Without_Weapon/Anim_Dead_1_Without_Weapon_Montage1.Anim_Dead_1_Without_Weapon_Montage1")
    (`KismetSystemLibrary.Delay` 1.0)
    (`self.K2_DestroyActor`)
    (else
      (set `self.Current Hit` (+ (`self.Current Hit`) 1)))))

(fn `BPIF_CheckIsEquipped?`
  (returns (`WeaponIsEquipped?` :type Boolean) (MuzzleTransform :type "Transform Structure"))
  (return false))

(fn `UserConstructionScript`)