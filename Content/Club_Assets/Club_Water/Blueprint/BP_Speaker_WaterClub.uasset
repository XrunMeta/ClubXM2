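; BP_Speaker_WaterClub is a club speaker that plays a playlist of songs on loop.
; BeginPlay binds the AudioComponent's finished and playback-percent delegates, then plays the song at SongID from Songlist.
; When a song finishes, SongID advances, wrapping to the start after the last entry.
; The playback-percent callback prints the song ID and elapsed time on screen as debug output.
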(event `PlaySong`
  ;[1 1 1] Play Song
  (`AudioComponent.SetSound` (`self.AudioComponent`) (`|GetArrayItem` (`self.Songlist`) (`self.SongID`)))
  (`AudioComponent.Play` (`self.AudioComponent`) 0.0))

(event `self.ReceiveBeginPlay`
  (bind _audiocomponent (`self.AudioComponent`))
  ;[1 1 1] Delegates on Begin Play and Play Song for the first time
  (add `AudioComponent.OnAudioPlaybackPercent` _audiocomponent (delegate `OnAudioPlaybackPercent_Event`))
  (add `AudioComponent.OnAudioFinished` _audiocomponent (delegate `OnAudioFinished_Event`))
  (`self.PlaySong`))

(event `SongFinishedPlaying`
  ;[1 1 1] Song is finished playing, play next song and repeat playlist
  (if (== (`self.SongID`) (`KismetArrayLibrary.Array_LastIndex` (`self.Songlist`)))
    (set `self.SongID` 0)
    (else
      (`/Engine/EditorBlueprintResources/StandardMacros.IncrementInt` (`self.SongID`)
        (:`  `
          _))))
  (`self.PlaySong`))

(event `OnAudioFinished_Event`
  ;[1 1 1] Delegates on Begin Play and Play Song for the first time
  (`self.SongFinishedPlaying`))

(event `OnAudioPlaybackPercent_Event`
  (params (PlayingSoundWave :type "SoundWave Object Reference") (PlaybackPercent :type "Float (single-precision)"))
  ;[1 1 1] Delegates on Begin Play and Play Song for the first time
  (`KismetSystemLibrary.PrintString` (`KismetStringLibrary.Concat_StrStr` "Song ID: " (`KismetStringLibrary.Conv_IntToString` (`self.SongID`)) " - " (`KismetStringLibrary.Conv_DoubleToString` (* PlaybackPercent (`SoundBase.Duration` PlayingSoundWave)))) true true (struct :`R` 1.0 :`B` 0.049349 :`A` 1.0) 0.0))

(fn `UserConstructionScript`)