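; Gameplay GameMode that handles player login, logout and character spawning for desktop and VR players.
; Login and logout update BP_GameState and a connected-controller list, which feeds chat name entries and removals.
; Spawning picks a random tagged PlayerStart, then possesses the chosen character, reopening MainWorld if that fails, or a VR character.
; VR spawn transforms are offset by inverse HMD location and yaw.
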(event `self.ReceiveTick`
  (params (DeltaSeconds :type "Float (single-precision)")))

(event `self.K2_PostLogin`
  (params (NewPlayer :type "PlayerController Object Reference"))
  (`self.PostLoginEvent` NewPlayer))

(event `PostLoginEvent`
  (params (`New Player` :type "PlayerController Object Reference"))
  (bind _asbp_game_state (cast `/Game/Blueprints/GameState/BP_GameState` (`GameplayStatics.GetGameState`)))
  (bind _output_get (set `self.As BP Game State` _asbp_game_state))
  (`/Engine/EditorBlueprintResources/StandardMacros.IsValid` _output_get
    (:`Is Valid`
      (`/Game/Blueprints/GameState/BP_GameState.Server_RegisterPlayerState` _output_get (`Controller.PlayerState` `New Player`))
      ;[0 1 0.184] Advanced Chat
      (bind _asbp_player_controller (cast `/Game/Blueprints/PlayerController/BP_PlayerController` `New Player`))
      (`KismetArrayLibrary.Array_AddUnique` (`self.ConnectedPlayers`) _asbp_player_controller)
      (`/Game/Blueprints/PlayerController/BP_PlayerController.SetPlayerName` _asbp_player_controller (`|GetArrayItem` (`self.PlayerNames`))))))

(event `PassPlayerName`
  (params (NewParam :type String))
  ;[0 1 0.184] Advanced Chat
  (for _array_element (`self.ConnectedPlayers`)
    (`/Game/Blueprints/PlayerController/BP_PlayerController.SetEntryPlayers` _array_element NewParam _array_element)))

(event `self.K2_OnLogout`
  (params (ExitingController :type "Controller Object Reference"))
  (bind _as_bp_game_state (`self.As BP Game State`)
    (:`then`
      (`/Game/Blueprints/GameState/BP_GameState.Server_PlayerLogout` _as_bp_game_state (`Controller.PlayerState` ExitingController))
      ;[1 1 1] Advance Chat
      (bind _asbp_player_controller (cast `/Game/Blueprints/PlayerController/BP_PlayerController` ExitingController))
      (bind _returnvalue (`KismetArrayLibrary.Array_RemoveItem` (`self.ConnectedPlayers`) _asbp_player_controller))
      (if _returnvalue
        (for _array_element (`self.ConnectedPlayers`)
          (`/Game/Blueprints/PlayerController/BP_PlayerController.DeletePlayerFromMessagesList(Client)` _array_element (`/Game/Blueprints/PlayerController/BP_PlayerController.PlayerName` _asbp_player_controller)))))
    (:`else`)))

(event `self.ReceiveEndPlay`
  (params (EndPlayReason :type "EEndPlayReason Enum" :default "Destroyed")))

(event `Spawn Character onServerTag location`
  (params (ServerTag :type Name) (`Character ID` :type Integer) (PlayerController :type "PlayerController Object Reference") (IsVR :type Boolean) (HMDOffset :type "Vector Structure") (HMDRotation :type "Rotator Structure"))
  ;[1 1 1] Spawn Character
  (if (not IsVR)
    (bind _outactors (`GameplayStatics.GetAllActorsOfClassWithTag` "/Script/Engine.PlayerStart" ServerTag))
    (bind _returnvalue (`|SpawnActorFromClass` (`|GetArrayItem` (`self.Character`) `Character ID`) (`KismetMathLibrary.MakeTransform` (`self.K2_GetActorLocation` (`|GetArrayItem` _outactors (`KismetMathLibrary.RandomIntegerInRange` 0 (- (`KismetArrayLibrary.Array_Length` _outactors) 1)))) (struct :`Yaw` -110.0)) "AdjustIfPossibleButAlwaysSpawn" "MultiplyWithRoot" PlayerController null))
    (`/Engine/EditorBlueprintResources/StandardMacros.IsValid` PlayerController
      (:`Is Valid`
        (`/Engine/EditorBlueprintResources/StandardMacros.IsValid` _returnvalue
          (:`Is Valid`
            (`Controller.Possess` PlayerController _returnvalue))
          (:`Is Not Valid`
            (`GameplayStatics.OpenLevelBySoftObjectPtr` "/Game/Maps/MainWorld.MainWorld" :!label _label))))
      (:`Is Not Valid`
        (goto _label)))
    (else
      (bind _outactors_2 (`GameplayStatics.GetAllActorsOfClassWithTag` "/Script/Engine.PlayerStart" ServerTag))
      (bind _returnvalue_2 (`|SpawnActorFromClass` "/Game/Blueprints/Character/BP_VRCharacter_ClubX_WidgetKeyborad.BP_VRCharacter_ClubX_WidgetKeyborad_C" (`KismetMathLibrary.ComposeTransforms` (`KismetMathLibrary.InvertTransform` (`KismetMathLibrary.MakeTransform` HMDOffset (`VRExpansionFunctionLibrary.GetHMDPureYaw` HMDRotation))) (`self.GetTransform` (`|GetArrayItem` _outactors_2 (`KismetMathLibrary.RandomIntegerInRange` 0 (- (`KismetArrayLibrary.Array_Length` _outactors_2) 1))))) "AdjustIfPossibleButAlwaysSpawn" "MultiplyWithRoot" null null))
      (`Controller.Possess` PlayerController _returnvalue_2))))

(fn `INFRefGameChatterAC`
  (returns (GameChatterAC :type "/Game/MultiplayerChatSys/Blueprint/Component/GameChatter_AC Object Reference"))
  (return null))

(fn `UserConstructionScript`)