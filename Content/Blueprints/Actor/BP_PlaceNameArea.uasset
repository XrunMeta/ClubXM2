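; BP_PlaceNameArea is an actor that displays a place name through a widget component.
; It casts the component's widget to WBP_PlaceName and sets its Name text from the PlaceName variable.
; The same update runs in both the construction script and BeginPlay, covering construction and the start of play.
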(event `self.ReceiveBeginPlay`
  (bind _aswbp_place_name (cast `/Game/Blueprints/Widgets/WBP_PlaceName` (`WidgetComponent.GetWidget` (`self.Widget`))))
  (`TextBlock.SetText` (`/Game/Blueprints/Widgets/WBP_PlaceName.Name` _aswbp_place_name) (`KismetTextLibrary.Conv_StringToText` (`self.Place Name`))))

(fn `UserConstructionScript`
  (bind _aswbp_place_name (cast `/Game/Blueprints/Widgets/WBP_PlaceName` (`WidgetComponent.GetWidget` (`self.Widget`))))
  (`TextBlock.SetText` (`/Game/Blueprints/Widgets/WBP_PlaceName.Name` _aswbp_place_name) (`KismetTextLibrary.Conv_StringToText` (`self.Place Name`))))