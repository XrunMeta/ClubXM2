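; Demo-room cover object that signals cover availability to overlapping actors in the TPS multiplayer pack.
; A CoverBox overlap sends the arrow's world rotation through CoverInterface on begin, and a zero rotation on end.
; A looping timer periodically hides the box, arrow and AI end-cover markers, then shows them again after a delay, making them blink.
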(event `self.ReceiveBeginPlay`
  (`KismetSystemLibrary.K2_SetTimerDelegate` (delegate `Loop`) 6.0 true))

(event `Loop`
  (`SceneComponent.SetVisibility` (`self.CoverBox1`) false false)
  (`SceneComponent.SetVisibility` (`|MakeArray` (`self.Arrow1`) (`self.AIEndCoverRight`) (`self.AIEndCoverLeft`) :!type "SceneComponent Object Reference") false false)
  (`KismetSystemLibrary.Delay` 3.0)
  (`SceneComponent.SetVisibility` (`self.CoverBox1`) true false)
  (`SceneComponent.SetVisibility` (`|MakeArray` (`self.Arrow1`) (`self.AIEndCoverRight`) (`self.AIEndCoverLeft`) :!type "SceneComponent Object Reference") true false))

(event `self.CoverBox1.OnComponentBeginOverlap`
  (params (OverlappedComponent :type "PrimitiveComponent Object Reference") (OtherActor :type "Actor Object Reference") (OtherComp :type "PrimitiveComponent Object Reference") (OtherBodyIndex :type Integer) (bFromSweep :type Boolean) (SweepResult :type "HitResult Structure (by ref)"))
  ;[1 1 1] Begin Overlap
  (if (`KismetSystemLibrary.DoesImplementInterface` OtherActor (`self.CoverInterface`))
    (message `/Game/TPS_Multiplayer_Pack/Blueprints/Interfaces/Cover_Interface.IsCoverAvaliable` OtherActor (`SceneComponent.K2_GetComponentRotation` (`self.Arrow1`)))))

(event `self.CoverBox1.OnComponentEndOverlap`
  (params (OverlappedComponent :type "PrimitiveComponent Object Reference") (OtherActor :type "Actor Object Reference") (OtherComp :type "PrimitiveComponent Object Reference") (OtherBodyIndex :type Integer))
  ;[1 1 1] End Overlap
  (if (`KismetSystemLibrary.DoesImplementInterface` OtherActor (`self.CoverInterface`))
    (message `/Game/TPS_Multiplayer_Pack/Blueprints/Interfaces/Cover_Interface.IsCoverAvaliable` OtherActor (struct))))

(fn `UserConstructionScript`)