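; Player state for a multiplayer game that syncs each player's profile, chosen character mesh and social messages between client and server.
; A delayed client event copies GameInstance data to the server, applies the DT_CharacterMesh mesh and requests a GameMode spawn by server tag, skipped on name changes.
; Client events update the HUD's player list, logout log and friend notifications.
; Server RPCs relay friend requests and work-in-progress chat through GameState interfaces.
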(event `self.ReceiveBeginPlay`
  (bind _asbp_game_instance (cast `/Game/Blueprints/Subsystem/BP_GameInstance` (`GameplayStatics.GetGameInstance`)))
  (set `self.As BP Game Instance` _asbp_game_instance)
  (bind _asbp_player_controller (cast `/Game/Blueprints/PlayerController/BP_PlayerController` (`self.GetPlayerController`)))
  (bind _asbp_gameplay_hud (cast `/Game/Blueprints/HUD/BP_GameplayHUD` (`PlayerController.GetHUD` _asbp_player_controller)))
  (set `self.As BP Gameplay HUD` _asbp_gameplay_hud)
  (bind _outrownames (`DataTableFunctionLibrary.GetDataTableRowNames` "/Game/Blueprints/DataTable/DT_CharacterMesh.DT_CharacterMesh"))
  (set `self.CharacterMeshes` _outrownames))

(event `Client_SetPlayerName`
  (params (PlayerState :type "PlayerState Object Reference"))
  (`KismetSystemLibrary.Delay` 0.1) ; Server faster than BeginPlay, to reduce casting, we need Delay 0.1s
  (bind _as_bp_game_instance (`self.As BP Game Instance`)
    (:`then`
      (`|ExecutionSequence`
        (:`then_0`
          (bind (_playerstate _playername _nickname _phonenumber _gender _idbackend _country _countrycode _region _status _wallet _datejoin _islockable _email _phonecode _uuid _characterid) (break `/Game/Blueprints/Structure/S_PlayerData` (`/Game/Blueprints/Subsystem/BP_GameInstance.PlayerDataStruct` _as_bp_game_instance)))
          (bind _s_playerdata (make `/Game/Blueprints/Structure/S_PlayerData` PlayerState _playername _nickname _phonenumber _gender _idbackend _country _countrycode _region _status _wallet _datejoin _islockable _email _phonecode _uuid _characterid))
          (set `/Game/Blueprints/Subsystem/BP_GameInstance.PlayerDataStruct` _s_playerdata (`self.As BP Game Instance`))
          (`self.Server_SendPlayerData` _s_playerdata)
          (bind _returnvalue (`|GetDataTableRow` "/Game/Blueprints/DataTable/DT_CharacterMesh.DT_CharacterMesh" (`|GetArrayItem` (`self.CharacterMeshes`) (- (`.CharacterID_100_C8C319B9430DBB60D97A3480207BB08F` (break `/Game/Blueprints/Structure/S_PlayerData` (`/Game/Blueprints/Subsystem/BP_GameInstance.PlayerDataStruct` (`self.As BP Game Instance`)))) 1)))
            (:`then`
              (message `/Game/Blueprints/Interface/BPI_CharacterSelect.BPIF_ApplyCharacterSelect` (`GameplayStatics.GetPlayerCharacter` 0) (`.SkeletalMesh_2_4EA27E1F4AFD66FCF62FC89336CD0CFD` (break `/Game/Blueprints/Structure/S_CharacterMesh` _returnvalue)))
              (message `/Game/Blueprints/Interface/BPI_CharacterSelect.BPIF_CancelCharacterSelect` (`self.As BP Gameplay HUD`) null)
              (`self.SR_Send_ServerTag` (`/Game/Blueprints/Subsystem/BP_GameInstance.ServerTag` (`self.As BP Game Instance`)) (`self.IsChangeName`)))))
        (:`then_1`
          (`KismetSystemLibrary.Delay` 0.5)
          (`self.OnSendPlayerData` _s_playerdata))))
    (:`else`)))

(event `Client_RetrievePlayerData`
  (params (PlayerData :type "Array of /Game/Blueprints/Structure/S_PlayerData Structure"))
  (bind _as_bp_gameplay_hud (`self.As BP Gameplay HUD`)
    (:`then`
      (`/Game/Blueprints/HUD/BP_GameplayHUD.UpdateListPlayers` _as_bp_gameplay_hud PlayerData))
    (:`else`)))

(event `Server_SendPlayerData`
  (params (PlayerData :type "/Game/Blueprints/Structure/S_PlayerData Structure"))
  (set `self.PlayerDataStruct` PlayerData))

(event `Client_PlayerLogout`
  (params (PlayerData :type "Array of /Game/Blueprints/Structure/S_PlayerData Structure"))
  (bind _as_bp_gameplay_hud (`self.As BP Gameplay HUD`)
    (:`then`
      (`/Game/Blueprints/HUD/BP_GameplayHUD.UpdateLogActivity` _as_bp_gameplay_hud PlayerData false))
    (:`else`)))

(event `SR_Send_ServerTag`
  (params (ServerTag :type Name) (IsChangeName :type Boolean))
  (bind ((`PlayerState_97_E5997660489A2A7EEEE909AD13D4D6C7` _playerstate) (`CharacterID_100_C8C319B9430DBB60D97A3480207BB08F` _characterid)) (break `/Game/Blueprints/Structure/S_PlayerData` (`self.PlayerDataStruct`)))
  (bind _returnvalue (`self.GetPlayerController` _playerstate))
  (if (not IsChangeName)
    (bind _asbp_gameplay_game_mode (cast `/Game/Blueprints/GameMode/BP_GameplayGameMode` (`GameplayStatics.GetGameMode`)))
    (`/Engine/EditorBlueprintResources/StandardMacros.IsValid` _asbp_gameplay_game_mode
      (:`Is Valid`
        (`/Engine/EditorBlueprintResources/StandardMacros.IsValid` _returnvalue
          (:`Is Valid`
            (`/Game/Blueprints/GameMode/BP_GameplayGameMode.Spawn Character onServerTag location` _asbp_gameplay_game_mode ServerTag _characterid _returnvalue)))))
    (else
      (set `self.IsChangeName` false))))

(event `Client_SendFriendsRequest`
  (params (ReceiverPlayer :type "/Game/Blueprints/Structure/S_PlayerData Structure") (SenderPlayer :type "/Game/Blueprints/Structure/S_PlayerData Structure"))
  (`/Game/Blueprints/HUD/BP_GameplayHUD.ActivateNotificationRequest` (cast `/Game/Blueprints/HUD/BP_GameplayHUD` (`PlayerController.GetHUD` (`self.GetPlayerController`)) :!pure true) ReceiverPlayer))

(event `/Game/Blueprints/Interface/BPI_InteractionInterface.FriendsRequestNotification`
  (params (ReceiverDataPlayer :type "/Game/Blueprints/Structure/S_PlayerData Structure"))
  (`self.Server_ReqFriends` ReceiverDataPlayer))

(event `Server_ReqFriends`
  (params (Receiver :type "/Game/Blueprints/Structure/S_PlayerData Structure"))
  (message `/Game/Blueprints/Interface/BPI_InteractionInterface.FriendsRequestNotification` (`GameplayStatics.GetGameState`) Receiver))

(event `SR_Message`
  (params (`Recv PlayerData` :type "/Game/Blueprints/Structure/S_PlayerData Structure"))
  ;[1 0.75 0] WIP In Local (from WBP), Run RPC on server of the Playerstate and run Interface in Gamestate
  (message `/Game/Blueprints/Interface/BPI_InteractionInterface.BPIF Chat Send Message` (`GameplayStatics.GetGameState`) `Recv PlayerData`))

(event `/Game/Blueprints/Interface/BPI_InteractionInterface.BPIF Chat Send Message`
  (params (Rec_DataPlayer :type "/Game/Blueprints/Structure/S_PlayerData Structure"))
  ;[1 0.75 0] WIP In Local (from WBP), Run RPC on server of the Playerstate and run Interface in Gamestate
  (`self.SR_Message` Rec_DataPlayer))

(event `OC_SendMessage`
  (params (PlayerName :type String))
  ;[1 0.75 0] WIP Receive message sent from GameState-Serverside
  (bind _returnvalue (`|CreateWidget` "/Game/Blueprints/Widgets/WBP_TriDebug_Text.WBP_TriDebug_Text_C" (`self.GetPlayerController`) (`|FormatText` "Beb {name}" (`KismetTextLibrary.Conv_StringToText` PlayerName))))
  (`PanelWidget.AddChild` (`/Game/Blueprints/Widgets/WBP_TriDebug.VerticalBox_Players` (`/Game/Blueprints/Widgets/WBP_MainWidget.WBP_TriDebug` (`/Game/Blueprints/HUD/BP_GameplayHUD.BP_MainWidget` (cast `/Game/Blueprints/HUD/BP_GameplayHUD` (`PlayerController.GetHUD` (`self.GetPlayerController`)) :!pure true)))) _returnvalue))

(fn `UserConstructionScript`)