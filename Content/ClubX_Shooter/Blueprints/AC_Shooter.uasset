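; AC_Shooter is a shooter component that handles equipping a weapon for the player character.
; EquipWeapon calls MCSwitchWeapon, which plays the standing rifle equip montage on player character 0 and toggles the WeaponEquipped flag, printing debug strings along the way.
; Disconnected montage and authority-switch nodes and an unused SelectedWeaponID variable remain, and nothing happens on BeginPlay or Tick.
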(event `self.ReceiveBeginPlay`)

(event `MC Switch Weapon`
  (`Character.PlayAnimMontage` (`GameplayStatics.GetPlayerCharacter` 0) "/Game/TPS_Multiplayer_Pack/Characters/Animations/Anim_Montages/Equip_Rifle_Standing_Montage.Equip_Rifle_Standing_Montage" 1.0 "None")
  (`KismetSystemLibrary.PrintString` "Equip Weapon")
  (if (`self.WeaponEquipped?`)
    (bind _output_get (set `self.WeaponEquipped?` false))
    (`KismetSystemLibrary.PrintString` (`KismetStringLibrary.Conv_BoolToString` _output_get))
    (else
      (bind _output_get_2 (set `self.WeaponEquipped?` true))
      (`KismetSystemLibrary.PrintString` (`KismetStringLibrary.Conv_BoolToString` _output_get_2)))))

(event `EquipWeapon`
  (`self.MC Switch Weapon`))