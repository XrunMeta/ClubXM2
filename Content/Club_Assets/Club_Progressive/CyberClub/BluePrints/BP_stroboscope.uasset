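; Strobe light actor for the cyber club that flashes a point light on and off.
; The construction script hides the light, and BeginPlay starts a fast looping timer on a custom event.
; That event uses two chained delays to show the light briefly, then hide it.
; The timer fires faster than the delays finish, so the delays effectively set the flash rhythm.
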(event `self.ReceiveTick`
  (params (DeltaSeconds :type "Float (single-precision)")))

(event `self.ReceiveBeginPlay`
  (`KismetSystemLibrary.K2_SetTimerDelegate` (delegate `CustomEvent`) 0.02 true))

(event `CustomEvent`
  (`KismetSystemLibrary.Delay` 0.15)
  (`SceneComponent.SetVisibility` (`self.PointLight`) true false)
  (`KismetSystemLibrary.Delay` 0.05)
  (`SceneComponent.SetVisibility` (`self.PointLight`) false false))

(fn `UserConstructionScript`
  (`SceneComponent.SetVisibility` (`self.PointLight`) false false))