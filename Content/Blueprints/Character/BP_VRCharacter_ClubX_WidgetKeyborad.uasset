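; VR player character for ClubX with an in-world keyboard for typing into login, signup and settings widgets.
; Keyboard presses append to the selected field, and Backspace clears it entirely.
; MainWorld disables movement; other levels enable walking and let alternate right grip toggle the phone, settings and keyboard.
; Tick feeds headset and controller transforms to the body AnimBP, while PlayerState data goes to the server, updating name display and GameState on replication.
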(event `ButtonEvent_Event`
  (params (Text :type Text) (Pressed :type Boolean) (KeyType :type "/Game/VRE/Level/Keyboard/KeyboardKeyTableRow Structure"))
  (if Pressed
    (switch `/Game/VRE/Level/Keyboard/SpecialKeyType` (`.KeyEvent_31_882B04C64F14DEBDB02F7D9F692CCF0F` (break `/Game/VRE/Level/Keyboard/KeyboardKeyTableRow` KeyType))
      (:`NewEnumerator10`
        (`self.InputText` Text)
        (`KismetSystemLibrary.PrintString` (`KismetTextLibrary.Conv_TextToString` Text) false))
      (:`NewEnumerator5`
        (`self.ClearText`)))))

(event `OnSendPlayerData_Event`
  (params (PlayerData :type "/Game/Blueprints/Structure/S_PlayerData Structure"))
  (`self.Server_GetPlayerDataStruct` PlayerData)
  (`KismetSystemLibrary.PrintString` "3. PCharacter" false true (struct :`G` 0.66 :`B` 1.0 :`A` 1.0) 20.0))

(event `Server_GetPlayerDataStruct`
  (params (PlayerData :type "/Game/Blueprints/Structure/S_PlayerData Structure"))
  (set `self.PlayerData` PlayerData))

(event `self.ReceiveBeginPlay`
  (bind _handmesh_right (`self.HandMesh-Right`))
  (bind _keyboarddatatable (`self.KeyboardDataTable`))
  (bind _vrmovementreference (`self.VRMovementReference`))
  (bind _bis3dkeyboard (`self.bIs3DKeyboard`))
  (bind _widgetkeyboard (`self.WidgetKeyboard`))
  (`parent.ReceiveBeginPlay`)
  (bind _asue4_abp_manny (cast `/Game/Characters/Mannequin_UE4/Animations/UE4_ABP_Manny` (`SkeletalMeshComponent.GetAnimInstance` (`self.Mesh`))))
  (set `self.As UE4 ABP Manny` _asue4_abp_manny)
  (`SceneComponent.SetHiddenInGame` _handmesh_right true false)
  (`SceneComponent.SetHiddenInGame` (`self.HandMesh-Left`) true false)
  (`SceneComponent.SetVisibility` _handmesh_right false false)
  (`SceneComponent.SetVisibility` (`self.HandMesh-Left`) false false)
  (`|ExecutionSequence`
    (:`then_0`
      (`SceneComponent.SetVisibility` _widgetkeyboard (not _bis3dkeyboard) false)
      (if _bis3dkeyboard
        (`/Game/VRE/Level/Keyboard/3DKeyboard.InitKeyboard` (`self.3DKeyboard`) _keyboarddatatable)
        (else
          (bind _as2dkeyboard (cast `/Game/VRE/Level/Keyboard/2DKeyboard` (`WidgetComponent.GetUserWidgetObject` _widgetkeyboard)))
          (bind _newsize (`/Game/VRE/Level/Keyboard/2DKeyboard.InitKeyboard` _as2dkeyboard _keyboarddatatable))
          (`WidgetComponent.SetDrawSize` _widgetkeyboard _newsize)
          (add `/Game/VRE/Level/Keyboard/2DKeyboard.ButtonEvent` _as2dkeyboard (delegate `ButtonEvent_Event`)))))
    (:`then_1`
      (bind _asbp_player_state (cast `/Game/Blueprints/PlayerState/BP_PlayerState` (`self.PlayerState`)))
      (bind _output_get (set `self.As BP Player State` _asbp_player_state))
      (add `/Game/Blueprints/PlayerState/BP_PlayerState.OnSendPlayerData` _output_get (delegate `OnSendPlayerData_Event`))
      (bind _asbp_game_instance (cast `/Game/Blueprints/Subsystem/BP_GameInstance` (`GameplayStatics.GetGameInstance`)))
      (set `self.As BP Game Instance` _asbp_game_instance))
    (:`then_2`
      (bind _aswbp_login (cast `/Game/Blueprints/Widgets/WBP_Login` (`WidgetComponent.GetUserWidgetObject` (`self.WidgetLogin`))))
      (set `self.As WBP Login` _aswbp_login)
      (bind _aswbp_settings (cast `/Game/Blueprints/Widgets/WBP_Settings` (`WidgetComponent.GetUserWidgetObject` (`self.WidgetSettings`))))
      (set `self.As WBP Settings` _aswbp_settings)
      (add `/Game/Blueprints/Widgets/WBP_Settings.OnGetInputKeyboard` _aswbp_settings (delegate `OnGetInputKeyboard_Event`))
      (bind _returnvalue (`GameplayStatics.GetCurrentLevelName` true))
      (if (`KismetStringLibrary.Contains` _returnvalue "MainWorld")
        (`CharacterMovementComponent.DisableMovement` _vrmovementreference)
        (else
          (`SceneComponent.SetHiddenInGame` (`self.Iphone`) true false)
          (`SceneComponent.SetHiddenInGame` (`self.WidgetLogin`) true false)
          (`SceneComponent.SetHiddenInGame` (`self.WidgetKeyboard`) true false)
          (`CharacterMovementComponent.SetMovementMode` _vrmovementreference "MOVE_Walking" 0))))))

(event `self.ReceiveTick`
  (params (DeltaSeconds :type "Float (single-precision)"))
  (`parent.ReceiveTick` DeltaSeconds)
  (bind _as_ue4_abp_manny (`self.As UE4 ABP Manny`)
    (:`then`
      (set `/Game/Characters/Mannequin_UE4/Animations/UE4_ABP_Manny.HeadTransform` (`SceneComponent.K2_GetComponentToWorld` (`self.VRReplicatedCamera`)) _as_ue4_abp_manny)
      (set `/Game/Characters/Mannequin_UE4/Animations/UE4_ABP_Manny.LeftTransform` (`SceneComponent.K2_GetComponentToWorld` (`self.LeftMotionController`)) _as_ue4_abp_manny)
      (set `/Game/Characters/Mannequin_UE4/Animations/UE4_ABP_Manny.RightTransform` (`SceneComponent.K2_GetComponentToWorld` (`self.RightMotionController`)) _as_ue4_abp_manny))
    (:`else`)))

(event `OnGetInputKeyboard_Event`
  (`SceneComponent.SetVisibility` (`self.WidgetKeyboard`) false false))

(event `EnhancedInput|/Game/VRE/Input/Actions/AlternateGripRight`
  (params (ActionValue :type Boolean) (ElapsedSeconds :type "Float (double-precision)") (TriggeredSeconds :type "Float (double-precision)") (InputAction :type "InputAction Object Reference" :default "/Game/VRE/Input/Actions/AlternateGripRight.AlternateGripRight"))
  (bind _iphone (`self.Iphone`))
  (:`Started`
    (bind _returnvalue (`GameplayStatics.GetCurrentLevelName` true))
    (if (not (`KismetStringLibrary.Contains` _returnvalue "MainWorld"))
      (`/Engine/EditorBlueprintResources/StandardMacros.FlipFlop`
        (:`A`
          (`SceneComponent.SetHiddenInGame` _iphone false false)
          (`SceneComponent.SetHiddenInGame` (`self.WidgetSettings`) false false)
          (`SceneComponent.SetHiddenInGame` (`self.WidgetKeyboard`) false false))
        (:`B`
          (`SceneComponent.SetHiddenInGame` _iphone true false)
          (`SceneComponent.SetHiddenInGame` (`self.WidgetSettings`) true false)
          (`SceneComponent.SetHiddenInGame` (`self.WidgetKeyboard`) true false))))))

(event `ClearText`
  (bind _as_wbp_login (`self.As WBP Login`))
  (if (`SceneComponent.IsVisible` (`self.WidgetLogin`))
    (switch `/Game/Blueprints/Enum/EEditableText` (`/Game/Blueprints/Widgets/WBP_Login.EditableText` _as_wbp_login)
      (:`NewEnumerator0`
        (`EditableText.SetText` (`/Game/Blueprints/Widgets/WBP_Login.InputEmail` _as_wbp_login) ""))
      (:`NewEnumerator1`
        (`EditableText.SetText` (`/Game/Blueprints/Widgets/WBP_Login.InputPassword` _as_wbp_login) ""))
      (:`NewEnumerator2`
        (`EditableText.SetText` (`/Game/Blueprints/Widgets/WBP_Login.SignupUsernames` _as_wbp_login) ""))
      (:`NewEnumerator3`
        (`EditableText.SetText` (`/Game/Blueprints/Widgets/WBP_Login.EmailSignUp` _as_wbp_login) ""))
      (:`NewEnumerator4`
        (`EditableText.SetText` (`/Game/Blueprints/Widgets/WBP_Login.SignupPassword` _as_wbp_login) ""))
      (:`NewEnumerator5`
        (`EditableText.SetText` (`/Game/Blueprints/Widgets/WBP_Login.SignUpPhoneNumber` _as_wbp_login) ""))
      (:`NewEnumerator10`
        (`EditableText.SetText` (`/Game/Blueprints/Widgets/WBP_Login.InputVerifCode_Signup` _as_wbp_login) "")))
    (else
      (`EditableText.SetText` (`/Game/Blueprints/Widgets/WBP_Settings.ConfirmPassword` (`self.As WBP Settings`)) ""))))

(event `InputText`
  (params (InText :type Text))
  (bind _as_wbp_login (`self.As WBP Login`))
  (bind _emailsignup (`/Game/Blueprints/Widgets/WBP_Login.EmailSignUp` _as_wbp_login))
  (bind _signuppassword (`/Game/Blueprints/Widgets/WBP_Login.SignupPassword` _as_wbp_login))
  (bind _signupusernames (`/Game/Blueprints/Widgets/WBP_Login.SignupUsernames` _as_wbp_login))
  (bind _inputverifcode_signup (`/Game/Blueprints/Widgets/WBP_Login.InputVerifCode_Signup` _as_wbp_login))
  (bind _confirmpassword (`/Game/Blueprints/Widgets/WBP_Settings.ConfirmPassword` (`self.As WBP Settings`)))
  (bind _inputemail (`/Game/Blueprints/Widgets/WBP_Login.InputEmail` _as_wbp_login))
  (bind _inputpassword (`/Game/Blueprints/Widgets/WBP_Login.InputPassword` _as_wbp_login))
  (bind _signupphonenumber (`/Game/Blueprints/Widgets/WBP_Login.SignUpPhoneNumber` _as_wbp_login))
  (set `self.DisplayText` InText)
  (if (`SceneComponent.IsVisible` (`self.WidgetLogin`))
    (switch `/Game/Blueprints/Enum/EEditableText` (`/Game/Blueprints/Widgets/WBP_Login.EditableText` _as_wbp_login)
      (:`NewEnumerator0`
        (`EditableText.SetText` _inputemail (`|FormatText` "{original}{addedText}" (`EditableText.Text` _inputemail) (`self.DisplayText`))))
      (:`NewEnumerator1`
        (`EditableText.SetText` _inputpassword (`|FormatText` "{original}{addedText}" (`EditableText.Text` _inputpassword) (`self.DisplayText`))))
      (:`NewEnumerator2`
        (`EditableText.SetText` _signupusernames (`|FormatText` "{original}{addedText}" (`EditableText.Text` _signupusernames) (`self.DisplayText`))))
      (:`NewEnumerator3`
        (`EditableText.SetText` _emailsignup (`|FormatText` "{original}{addedText}" (`EditableText.Text` _emailsignup) (`self.DisplayText`))))
      (:`NewEnumerator4`
        (`EditableText.SetText` _signuppassword (`|FormatText` "{original}{addedText}" (`EditableText.Text` _signuppassword) (`self.DisplayText`))))
      (:`NewEnumerator5`
        (`EditableText.SetText` _signupphonenumber (`|FormatText` "{original}{addedText}" (`EditableText.Text` _signupphonenumber) (`self.DisplayText`))))
      (:`NewEnumerator10`
        (`EditableText.SetText` _inputverifcode_signup (`|FormatText` "{original}{addedText}" (`EditableText.Text` _inputverifcode_signup) (`self.DisplayText`)))))
    (else
      (`EditableText.SetText` _confirmpassword (`|FormatText` "{original}{addedText}" (`EditableText.GetText` _confirmpassword) (`self.DisplayText`))))))

(fn `OnRep_PlayerData`
  (bind (_playerstate _playername) (break `/Game/Blueprints/Structure/S_PlayerData` (`self.PlayerData`)))
  (`TextRenderComponent.K2_SetText` (`self.PlayerNameDisplay`) (`KismetTextLibrary.Conv_StringToText` _playername))
  (`KismetSystemLibrary.PrintString` (`KismetStringLibrary.Concat_StrStr` "3. " _playername) false true (struct :`G` 0.66 :`B` 1.0 :`A` 1.0) 50.0)
  (bind _asbp_game_state (cast `/Game/Blueprints/GameState/BP_GameState` (`GameplayStatics.GetGameState`))
    (:`then`
      (`/Game/Blueprints/GameState/BP_GameState.Multicast_RetrievePlayerData` _asbp_game_state (`self.PlayerData`)))
    (:`CastFailed`
      (`KismetSystemLibrary.K2_SetTimer` null "OnRep_PlayerData" 0.1))))

(fn `UserConstructionScript`
  (`parent.UserConstructionScript`))