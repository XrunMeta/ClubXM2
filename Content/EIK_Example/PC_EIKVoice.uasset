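; Example player controller for EOS voice chat via EIK, with debug prints at each step.
; Chained async callbacks initialize, connect and log in, then fetch a room token with a hard-coded client IP, join and transmit, updating a voice widget's labels.
; Also handles Android mic permission, a music toggle and a key that lists input devices and Team1 players.
; Widget creation, leave-room and stop-transmit logic are unwired.
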(event `Key|One`
  (params (Key :type "Key Structure"))
  ;[1 1 1] Get All device
  (:`Pressed`
    (bind _returnvalue (`EVIK_Functions.GetInputMethods`))
    (for _array_element _returnvalue
      (bind (_id _displayname) (break `DeviceEVIKSettings` _array_element))
      (`KismetSystemLibrary.PrintText` (`|FormatText` "{id} - {displayname}" _id _displayname)))
    (`KismetSystemLibrary.Delay` 0.2)
    (bind _returnvalue_2 (`EVIK_Functions.GetPlayersInRoom` "Team1"))
    (for _array_element_2 _returnvalue_2
      (`KismetSystemLibrary.PrintString` _array_element_2))))

(event `ConnectToVoiceChat`
  (params (PlayerName :type String))
  ;[1 1 1] Connect to Voice by Player Name
  (`KismetSystemLibrary.PrintText` (`|FormatText` "Connecting voice as {name}" PlayerName))
  (bind _returnvalue (`EVIK_Functions.InitializeEOSVoiceChat`))
  (if _returnvalue
    (`KismetSystemLibrary.PrintString` "Initializing...")
    (`EVIK_Functions.ConnectVoiceChat` (delegate `ConnectToEOSVoiceChat_Result`))
    (else
      (`KismetSystemLibrary.PrintString` "Initializing EOS Failed"))))

(event `ConnectToEOSVoiceChat_Result`
  (params (bWasSuccess :type Boolean) (Result :type "EEVIKResultCodes Enum" :default "Success"))
  ;[1 1 1] Connect to Voice by Player Name
  (if bWasSuccess
    (`EVIK_Functions.LoginEOSVoiceChat` (stale `ConnectToVoiceChat` PlayerName) (delegate `LoginToEOSVoiceChat_Result`))
    (else
      (`KismetSystemLibrary.PrintString` "Connect to EOS Voice Failed"))))

(event `self.ReceiveBeginPlay`)

(event `LoginToEOSVoiceChat_Result`
  (params (bWasSuccess :type Boolean) (Result :type "EEVIKResultCodes Enum" :default "Success"))
  ;[1 1 1] Connect to Voice by Player Name
  (if bWasSuccess
    (`KismetSystemLibrary.PrintString` (`KismetStringLibrary.Concat_StrStr` "Logged in to Voice as: " (`EVIK_Functions.LoggedInUser`)))
    (`TextBlock.SetText` (`/Game/EIK_Example/WBP_EIKVoiceWidget.Text_PlayerName` (`self.As WBP EIK Voice Widget`)) (`KismetTextLibrary.Conv_StringToText` (`EVIK_Functions.LoggedInUser`)))
    (else
      (`KismetSystemLibrary.PrintString` "Login To EOS Voice Chat FAILED" true true (struct :`R` 1.0 :`G` 0.793158 :`A` 1.0) 5.0))))

(event `Key|Two`
  (params (Key :type "Key Structure"))
  ;[1 1 1] Leave Room
)

(event `CustomEvent`
  (params (bWasSuccess :type Boolean) (Result :type "EEVIKResultCodes Enum" :default "Success"))
  ;[1 1 1] Leave Room
  (if bWasSuccess
    (`KismetSystemLibrary.PrintString` "Bye Bye Voice")
    (else
      (`KismetSystemLibrary.PrintString` "Failed Leave Room"))))

(event `Req_VoicePermission`
  ;[1 1 1] Request permissions, if on mobile platform
  (switch `string` (`GameplayStatics.GetPlatformName`)
    (:`Default`
      (`KismetSystemLibrary.PrintString` "Not Android, Bypassing Permission Request"))
    (:`Android`
      (`KismetSystemLibrary.PrintString` "Requesting Android Voice Permission")
      (bind _returnvalue (`AndroidPermissionFunctionLibrary.CheckPermission` (`self.MicPermission`)))
      (if _returnvalue
        (`KismetSystemLibrary.PrintString` "Microphone Permission available." true true (struct :`G` 0.66 :`B` 1.0 :`A` 1.0) 10.0))))
  (`KismetSystemLibrary.Delay` 0.2)
  (`KismetSystemLibrary.PrintString` "Microphone Permission not available, starting request" true true (struct :`G` 0.66 :`B` 1.0 :`A` 1.0) 10.0)
  (bind _returnvalue_2 (`AndroidPermissionFunctionLibrary.AcquirePermissions` (`|MakeArray` (`self.MicPermission`))))
  (add `AndroidPermissionCallbackProxy.OnPermissionsGrantedDynamicDelegate` _returnvalue_2 (delegate `OnGranted`)))

(event `GetRoomToken`
  (params (RoomName :type String))
  (bind _output_get (set `self.Room Name` RoomName))
  (`EVIK_Functions.EOSRoomToken` _output_get (`EVIK_Functions.LoggedInUser`) "10.0.0.1" (delegate `GetEOSVoiceRoomToken_Result`)) ; 10.0.0.1
)

(event `GetEOSVoiceRoomToken_Result`
  (params (bWasSuccess :type Boolean) (RoomData :type String))
  (if bWasSuccess
    (`KismetSystemLibrary.PrintString` "Getting Voice Toket")
    (`EVIK_Functions.JoinEOSRoom` (`self.Room Name`) RoomData false (delegate `JoinEOSVoiceRoom_Result`))
    (else
      (`KismetSystemLibrary.PrintString` "Getting Voice Room Token Failed"))))

(event `OnGranted`
  (params (Permissions :type "Array of String (by ref)") (GrantResults :type "Array of Boolean (by ref)"))
  ;[1 1 1] Permission Request Callback
  (`KismetSystemLibrary.PrintString` "Permission Request Callback received" true true (struct :`G` 0.66 :`B` 1.0 :`A` 1.0) 10.0)
  (for (_array_element _array_index) Permissions
    (`KismetSystemLibrary.PrintText` (`|FormatText` "GrantResult for {permission} is: {result}" _array_element (`|GetArrayItem` GrantResults _array_index)) true true (struct :`G` 0.66 :`B` 1.0 :`A` 1.0) 10.0)
    (if (`KismetStringLibrary.EqualEqual_StrStr` (`self.MicPermission`) _array_element)
      (`|ExecutionSequence`
        (:`then_0`
          (break)))))
  (`KismetSystemLibrary.PrintString` "Done Requesting Permission" true true (struct :`G` 0.013172 :`B` 1.0 :`A` 1.0) 5.0))

(event `JoinEOSVoiceRoom_Result`
  (params (bWasSuccess :type Boolean) (Result :type "EEVIKResultCodes Enum" :default "Success"))
  (if bWasSuccess
    (`KismetSystemLibrary.PrintString` "Join EOS Voice Room Success" true true (struct :`G` 0.080223 :`B` 1.0 :`A` 1.0) 5.0)
    (bind _returnvalue (`EVIK_Functions.GetAllRooms`))
    (for _array_element _returnvalue
      (`KismetSystemLibrary.PrintString` _array_element true true (struct :`G` 0.018708 :`B` 1.0 :`A` 1.0) 5.0))
    (`KismetSystemLibrary.Delay` 0.2)
    (bind _returnvalue_2 (`EVIK_Functions.TransmitToSelectedRoom` (`self.Room Name`)))
    (if _returnvalue_2
      (`KismetSystemLibrary.PrintString` "Transmit Voice READY" true true (struct :`G` 0.018708 :`B` 1.0 :`A` 1.0) 5.0)
      (`TextBlock.SetText` (`/Game/EIK_Example/WBP_EIKVoiceWidget.Text_RoomName` (`self.As WBP EIK Voice Widget`)) (`KismetTextLibrary.Conv_StringToText` (`self.Room Name`)))
      (else
        (`KismetSystemLibrary.PrintString` "Failed Transmit voice")))
    (else
      (`KismetSystemLibrary.PrintString` "Join EOS Voice Room Failed"))))

(event `ToggleMusic`
  (if (`self.MusicON`)
    (`AudioComponent.Stop` (`self.Music`))
    (set `self.MusicON` false)
    (else
      (`/Engine/EditorBlueprintResources/StandardMacros.IsValid` (`self.Music`)
        (:`Is Valid`
          _)
        (:`Is Not Valid`
          (bind _returnvalue (`GameplayStatics.SpawnSound2D` null 0.05 1.0 0.0 null))
          (set `self.Music` _returnvalue)))
      (`AudioComponent.Play` (`self.Music`) 0.0)
      (set `self.MusicON` true))))

(fn `UserConstructionScript`)