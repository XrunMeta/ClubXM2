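; Shotgun projectile Blueprint for a third-person shooter multiplayer pack that deals damage on impact.
; When its Bullet component hits an actor implementing DamageInterface, it sends TakeDamageMessage with damage range, crit chance, hit bone, instigator and a force-scaled impact vector.
; It destroys itself after a brief delay on any hit, damageable or not.
; The construction script only calls the parent.
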(event `self.Bullet.OnComponentHit`
  (params (HitComponent :type "PrimitiveComponent Object Reference") (OtherActor :type "Actor Object Reference") (OtherComp :type "PrimitiveComponent Object Reference") (NormalImpulse :type "Vector Structure") (Hit :type "HitResult Structure (by ref)"))
  (bind (_bblockinghit _binitialoverlap _time _distance _location _impactpoint _normal _impactnormal _physmat _hitactor _hitcomponent _hitbonename _bonename _hititem _elementindex _faceindex _tracestart _traceend) (`GameplayStatics.BreakHitResult` Hit))
  (if (`KismetSystemLibrary.DoesImplementInterface` _hitactor "/Game/TPS_Multiplayer_Pack/Blueprints/Interfaces/DamageInterface.DamageInterface_C")
    (message `/Game/TPS_Multiplayer_Pack/Blueprints/Interfaces/DamageInterface.TakeDamage` _hitactor (`self.DamageMin`) (`self.DamageMax`) (`self.CritChance`) _hitbonename (`self.GetInstigator`) (* (`KismetMathLibrary.Normal` (`KismetMathLibrary.GetDirectionUnitVector` _tracestart _traceend)) (`self.ImpactForce`)))
    (`KismetSystemLibrary.Delay` 0.03)
    (`self.K2_DestroyActor`)
    (else
      (`KismetSystemLibrary.Delay` 0.03)
      (`self.K2_DestroyActor`))))

(fn `UserConstructionScript`
  (`parent.UserConstructionScript`))