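; Multiplayer touch-controlled player avatar that can jump, dance, teleport via lifts, sit on chairs and open interaction menus on tapped players or NPCs.
; BeginPlay binds HUD buttons and player-state data, with actions applied locally and through server events.
; Right-half swipes rotate the camera, while Tick traces under the finger for taps and turns the username widget toward the camera.
; OnRep_PlayerData multicasts via GameState and updates that username, retrying by timer until ready.
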(event `ActivateDancing`
  (bind _charactermovement (`self.CharacterMovement`))
  ;[1 1 1] Server Dancing
  (if (`self.IsDancing`)
    (set `self.IsDancing` false)
    (`CharacterMovementComponent.SetMovementMode` _charactermovement "MOVE_Walking" 0)
    (else
      (set `self.IsDancing` true)
      (`self.Server_Dancing` (`KismetMathLibrary.RandomInteger` 8))
      (`CharacterMovementComponent.DisableMovement` _charactermovement))))

(event `Server_Dancing`
  (params (DanceID :type Integer))
  ;[1 1 1] Server Dancing
  (set `self.DanceID` DanceID)
  (`CharacterMovementComponent.DisableMovement` (`self.CharacterMovement`))
  (set `self.IsDancing` true))

(event `self.ReceiveBeginPlay`
  ;[0 0 0] Initialize
  (bind _aswbp_top_head_username (cast `/Game/Blueprints/Widgets/WBP_TopHeadUsername` (`WidgetComponent.GetUserWidgetObject` (`self.UsernameWidgetComp`)))
    (:`then`
      (`/Engine/EditorBlueprintResources/StandardMacros.IsValid` _aswbp_top_head_username
        (:`Is Valid`
          (set `self.As WBP Top Head Username` _aswbp_top_head_username)
          (bind _asbp_player_controller (cast `/Game/Blueprints/PlayerController/BP_PlayerController` (`self.GetController`)))
          (bind _output_get (set `self.As BP Player Controller` _asbp_player_controller))
          (bind _asbp_gameplay_hud (cast `/Game/Blueprints/HUD/BP_GameplayHUD` (`PlayerController.GetHUD` _output_get)))
          (bind _output_get_2 (set `self.As BP Gameplay HUD` _asbp_gameplay_hud))
          (bind _bp_mainwidget (`/Game/Blueprints/HUD/BP_GameplayHUD.BP_MainWidget` _output_get_2)
            (:`then`
              (add `/Game/Blueprints/Widgets/WBP_MainWidget.OnInteractingFinished` _bp_mainwidget (delegate `OnInteractingFinished_Event`))
              (bind _wbp_mainmenu (`/Game/Blueprints/Widgets/WBP_MainWidget.WBP_MainMenu` _bp_mainwidget)
                (:`then`
                  (bind _output_get_3 (set `self.WBP Main Menu` _wbp_mainmenu))
                  (add `Button.OnPressed` (`/Game/Blueprints/Widgets/WBP_MainMenu.ButtonInteract` _output_get_3) (delegate `InteractionButtonOnPressed_Event`))
                  (add `Button.OnPressed` (`/Game/Blueprints/Widgets/WBP_MainMenu.ButtonDance` _output_get_3) (delegate `DanceButtonOnPressed_Event`))
                  (bind _buttonjump (`/Game/Blueprints/Widgets/WBP_MainMenu.ButtonJump` _output_get_3))
                  (add `Button.OnPressed` _buttonjump (delegate `OnPressed_Event`))
                  (add `Button.OnReleased` _buttonjump (delegate `OnReleased_Event`))
                  (bind _asbp_player_state (cast `/Game/Blueprints/PlayerState/BP_PlayerState` (`self.PlayerState`)))
                  (bind _output_get_4 (set `self.As BP Player State` _asbp_player_state))
                  (add `/Game/Blueprints/PlayerState/BP_PlayerState.OnSendPlayerData` _output_get_4 (delegate `OnSendPlayerData_Event`)))
                (:`else`)))
            (:`else`)))
        (:`Is Not Valid`
          (`KismetSystemLibrary.PrintString` "WidgetComp Not Valid" :!label _label))))
    (:`CastFailed`
      (goto _label))))

(event `OnInteractingFinished_Event`
  ;[0 0 0] Initialize
  (set `self.IsInteracting` false))

(event `InteractionButtonOnPressed_Event`
  ;[0 0 0] Initialize
  (`self.InteractButtonOnPressed`))

(event `DanceButtonOnPressed_Event`
  ;[0 0 0] Initialize
  (`self.ActivateDancing`))

(event `OnPressed_Event`
  ;[0 0 0] Initialize
  (`self.Jump`))

(event `OnReleased_Event`
  ;[0 0 0] Initialize
  (`self.StopJumping`))

(event `OnSendPlayerData_Event`
  (params (PlayerData :type "/Game/Blueprints/Structure/S_PlayerData Structure"))
  ;[0 0 0] Initialize
  (`self.Server_GetPlayerDataStruct` PlayerData))

(event `Server_GetPlayerDataStruct`
  (params (PlayerData :type "/Game/Blueprints/Structure/S_PlayerData Structure"))
  ;[0 0 0] Initialize
  ;;[1 1 1] Server GetPlayerDataStruct
  (set `self.PlayerData` PlayerData))

(event `/Game/Blueprints/Interface/BPI_InteractionInterface.InteractableActor`
  (params (InteractableActor :type "/Game/Blueprints/Actor/BP_Interactable Object Reference"))
  ;[0 0 0] Interfaces
  (bind _output_get (set `self.ActorInteractable` InteractableActor))
  (`/Engine/EditorBlueprintResources/StandardMacros.IsValid` _output_get
    (:`Is Valid`
      (bind _output_get_2 (set `self.Interact Type` (`/Game/Blueprints/Actor/BP_Interactable.InteractType` _output_get)))
      (switch `/Game/Blueprints/Enum/EInteractActorType` _output_get_2
        (:`NewEnumerator0`
          (set `self.DestinationLocation` (`/Game/Blueprints/Actor/BP_Interactable.DestinationLocation` _output_get)))))))

(event `Server_LiftingPlayerToLocation`
  ;[0 0 0] Interaction
  ;;[1 1 1 1 15] Server Teleport
  (`self.K2_SetActorLocationAndRotation` (`self.DestinationLocation`) (struct :`Yaw` -180.0)))

(event `InteractButtonOnPressed`
  (bind _seatposition (`self.SeatPosition`))
  (bind _seatposition_2 (`self.SeatPosition`))
  ;[0 0 0] Interaction
  (`/Engine/EditorBlueprintResources/StandardMacros.IsValid` (`self.ActorInteractable`)
    (:`Is Valid`
      (switch `/Game/Blueprints/Enum/EInteractActorType` (`self.Interact Type`)
        (:`NewEnumerator0`
          (if (`self.IsPlayerTeleported`)
            (`KismetSystemLibrary.PrintString` "Wait a seconds!")
            (else
              (`self.Server_LiftingPlayerToLocation`)
              (`self.K2_SetActorLocationAndRotation` (`self.DestinationLocation`) (struct :`Yaw` -180.0))
              (set `self.IsPlayerTeleported` true)
              (`KismetSystemLibrary.Delay` 1.0)
              (set `self.IsPlayerTeleported` false))))
        (:`NewEnumerator1`
          (if (`self.IsSitting`)
            (`self.Server_StandUp`)
            (set `self.IsSitting` false) ; Stand Up
            (`CharacterMovementComponent.SetMovementMode` (`self.CharacterMovement`) "MOVE_Walking" 0)
            (`self.K2_SetActorLocationAndRotation` (`KismetMathLibrary.MakeVector` (+ (.x (.location _seatposition)) -50.0) (.y (.location _seatposition)) (.z (.location _seatposition))) (.rotation _seatposition))
            (bind _wbp_main_menu (`self.WBP Main Menu`)
              (:`then`
                (`Widget.SetVisibility` (`/Game/Blueprints/Widgets/WBP_MainMenu.BorderInteract` _wbp_main_menu) "Visible"))
              (:`else`))
            (else
              (`self.Server_SitDownPlayer`)
              (set `self.IsSitting` true) ; Sit Down
              (`CharacterMovementComponent.DisableMovement` (`self.CharacterMovement`))
              (`self.K2_SetActorLocationAndRotation` (`KismetMathLibrary.MakeVector` (.x (.location _seatposition_2)) (.y (.location _seatposition_2)) (+ (.z (.location _seatposition_2)) 50.0)) (.rotation _seatposition_2))
              (bind _wbp_main_menu_2 (`self.WBP Main Menu`)
                (:`then`
                  (`Widget.SetVisibility` (`/Game/Blueprints/Widgets/WBP_MainMenu.BorderInteract` _wbp_main_menu_2) "Collapsed"))
                (:`else`)))))))
    (:`Is Not Valid`
      (`KismetSystemLibrary.PrintString` "Interactable Actor is null"))))

(event `Server_StandUp`
  (bind _seatposition (`self.SeatPosition`))
  ;[0 0 0] Interaction
  ;;[1 1 1] Server Stand Up
  (set `self.IsSitting` false)
  (`CharacterMovementComponent.SetMovementMode` (`self.CharacterMovement`) "MOVE_Walking" 0)
  (`self.K2_SetActorLocationAndRotation` (`KismetMathLibrary.MakeVector` (+ (.x (.location _seatposition)) -50.0) (.y (.location _seatposition)) (.z (.location _seatposition))) (.rotation _seatposition)))

(event `/Game/Blueprints/Interface/BPI_InteractionInterface.InteractableCharacter`
  (params (Player :type "Actor Object Reference"))
  ;[0 0 0] Interfaces
  (if (`self.IsInteracting`)
    (`KismetSystemLibrary.PrintString` "Still Interacting")
    (else
      (set `self.IsInteracting` true)
      (cast `/Game/Blueprints/Character/BP_PlayerCharacter` Player ; Just in case if we need their data like PlayerDataStruct
        (:`then`
          (bind _as_bp_gameplay_hud (`self.As BP Gameplay HUD`)
            (:`then`
              (bind _bp_mainwidget (`/Game/Blueprints/HUD/BP_GameplayHUD.BP_MainWidget` _as_bp_gameplay_hud)
                (:`then`
                  (`/Game/Blueprints/Widgets/WBP_MainWidget.ActivateCharacterOpponentMenu` _bp_mainwidget false))
                (:`else`)))
            (:`else`)))
        (:`CastFailed`
          (cast `/Game/Blueprints/Character/BP_BaseNPC` Player) ; Just in case if we need NPC data
          (bind _as_bp_gameplay_hud_2 (`self.As BP Gameplay HUD`)
            (:`then`
              (bind _bp_mainwidget_2 (`/Game/Blueprints/HUD/BP_GameplayHUD.BP_MainWidget` _as_bp_gameplay_hud_2)
                (:`then`
                  (`/Game/Blueprints/Widgets/WBP_MainWidget.ActivateCharacterOpponentMenu` _bp_mainwidget_2 true))
                (:`else`)))
            (:`else`)))))))

(event `InputTouch`
  (params (Location :type "Vector Structure") (FingerIndex :type "ETouchIndex Enum"))
  (bind _returnvalue (>= Location_X (/ (`KismetMathLibrary.BreakVector2D` (`WidgetLayoutLibrary.GetViewportSize`)) 2.0)))
  ;[0 0 0] Swipe Control
  (:`Pressed`
    (if _returnvalue
      (set `self.Start Position` (`KismetMathLibrary.MakeVector2D` Location_X Location_Y) :!label _label_2)
      (set `self.ActiveFingerArea` FingerIndex)))
  (:`Released`
    (set `self.IsCamRotating` false)
    (goto _label_2))
  (:`Moved`
    (if _returnvalue
      (set `self.IsCamRotating` true)
      (`self.UpdateCamPosition` (`KismetMathLibrary.MakeVector2D` Location_X Location_Y))
      (goto _label_2))))

(event `Server_SitDownPlayer`
  (bind _seatposition (`self.SeatPosition`))
  ;[0 0 0] Interaction
  ;;[1 1 1] Server Seat Position
  (set `self.IsSitting` true)
  (`CharacterMovementComponent.DisableMovement` (`self.CharacterMovement`))
  (`self.K2_SetActorLocationAndRotation` (`KismetMathLibrary.MakeVector` (.x (.location _seatposition)) (.y (.location _seatposition)) (+ (.z (.location _seatposition)) 50.0)) (.rotation _seatposition)))

(event `UpdateCamPosition`
  (params (StartPosition :type "Vector2D Structure"))
  (bind _touchsensitivity (`self.TouchSensitivity`))
  (bind (_returnvalue_x _returnvalue_y) (`KismetMathLibrary.BreakVector2D` (- StartPosition (`self.Start Position`))))
  ;[0 0 0] Swipe Control
  (if (`|EnumEquality` (stale `InputTouch` FingerIndex) (`self.ActiveFingerArea`))
    (`self.AddControllerYawInput` (/ _returnvalue_x _touchsensitivity))
    (`self.AddControllerPitchInput` (/ _returnvalue_y _touchsensitivity))))

(event `self.ReceiveTick`
  (params (DeltaSeconds :type "Float (single-precision)"))
  (bind _usernamewidgetcomp (`self.UsernameWidgetComp`))
  ;[0 0 0] Set Rotation for Username Widget Comp to facing the player
  (`SceneComponent.K2_SetWorldRotation` _usernamewidgetcomp (`KismetMathLibrary.FindLookAtRotation` (`SceneComponent.K2_GetComponentLocation` _usernamewidgetcomp) (`self.K2_GetActorLocation` (`GameplayStatics.GetPlayerCameraManager` 0))) false false)
  ;[0 0 0] Tap Avatar (Player/NPC ) to open the radial menu widget
  (bind _as_bp_player_controller (`self.As BP Player Controller`)
    (:`then`
      (bind (_hitresult _returnvalue) (`PlayerController.GetHitResultUnderFingerForObjects` _as_bp_player_controller (`self.ActiveFingerArea`) (`|MakeArray` "ObjectTypeQuery3" :!type "EObjectTypeQuery Enum") true))
      (if _returnvalue
        (bind (_bblockinghit _binitialoverlap _time _distance _location _impactpoint _normal _impactnormal _physmat _hitactor) (`GameplayStatics.BreakHitResult` _hitresult))
        (if (!= _hitactor self)
          (if (not (`self.IsCamRotating`))
            (`/Game/Blueprints/Interface/BPI_InteractionInterface.InteractableCharacter` _hitactor)))))
    (:`else`)))

(event `EnhancedInput|/Game/ThirdPerson/Input/Actions/IA_Interact`
  (params (ActionValue :type Boolean) (ElapsedSeconds :type "Float (double-precision)") (TriggeredSeconds :type "Float (double-precision)") (InputAction :type "InputAction Object Reference" :default "/Game/ThirdPerson/Input/Actions/IA_Interact.IA_Interact"))
  (bind (_hitresult _returnvalue) (`PlayerController.GetHitResultUnderCursorForObjects` (`self.As BP Player Controller`) (`|MakeArray` "ObjectTypeQuery3" :!type "EObjectTypeQuery Enum") true))
  (bind (_bblockinghit _binitialoverlap _time _distance _location _impactpoint _normal _impactnormal _physmat _hitactor) (`GameplayStatics.BreakHitResult` _hitresult))
  ;[0 0 0] NOTE:: Debugging Purpose for tap avatar feature
  (:`Triggered`
    (if _returnvalue
      (if (!= _hitactor self)
        (`/Game/Blueprints/Interface/BPI_InteractionInterface.InteractableCharacter` _hitactor)))))

(fn `OnRep_PlayerData`
  (bind _asbp_game_state (cast `/Game/Blueprints/GameState/BP_GameState` (`GameplayStatics.GetGameState`))
    (:`then`
      (`/Game/Blueprints/GameState/BP_GameState.Multicast_RetrievePlayerData` _asbp_game_state (`self.PlayerData`))
      (bind _as_wbp_top_head_username (`self.As WBP Top Head Username`)
        (:`then`
          (`self.SetTopHeadUsername` _as_wbp_top_head_username))
        (:`else`
          (`KismetSystemLibrary.K2_SetTimer` null "OnRep_PlayerData" 0.1))))
    (:`CastFailed`
      (`KismetSystemLibrary.K2_SetTimer` null "OnRep_PlayerData" 0.1))))

(fn `SetTopHeadUsername`
  (params (WidgetComp :type "/Game/Blueprints/Widgets/WBP_TopHeadUsername Object Reference"))
  (`/Engine/EditorBlueprintResources/StandardMacros.IsValid` WidgetComp
    (:`Is Valid`
      (`/Game/Blueprints/Widgets/WBP_TopHeadUsername.SetUsername` WidgetComp (`KismetTextLibrary.Conv_StringToText` (`.PlayerName_95_43BA035F45A895FCE829889BE686CA1C` (break `/Game/Blueprints/Structure/S_PlayerData` (`self.PlayerData`))))))))

(fn `UserConstructionScript`)