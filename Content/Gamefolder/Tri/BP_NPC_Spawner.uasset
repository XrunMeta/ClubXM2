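; Spawner actor that spawns one BP_CharaNPC at its own transform on BeginPlay.
; After spawning, it calls SRChangeNPCMesh on the result of FCastToCharaNPC, which casts and caches player character 0 as BP_CharaNPC rather than using the spawned actor.
; Mesh randomization from NPCMeshArray and a DoN-gated spawn remain as unconnected nodes.
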(event `self.ReceiveBeginPlay`
  (`self.SpawnNPC`))

(event `SpawnNPC`
  (bind _returnvalue (`|SpawnActorFromClass` "/MultixOnline/Blueprints/BP_CharaNPC.BP_CharaNPC_C" (`self.GetTransform` self) "Undefined" "MultiplyWithRoot" null null))
  (bind _as_chara_npc (`self.FCastToCharaNPC`))
  (`/MultixOnline/Blueprints/BP_CharaNPC.SR_ChangeNPCMesh` _as_chara_npc))

(event `self.ReceiveTick`
  (params (DeltaSeconds :type "Float (single-precision)")))

(fn `FCastToCharaNPC`
  (returns (`As Chara NPC` :type "/MultixOnline/Blueprints/BP_CharaNPC Object Reference"))
  (`self.As BP Chara NPC`
    (:`then`
      _)
    (:`else`
      (bind _asbp_chara_npc (cast `/MultixOnline/Blueprints/BP_CharaNPC` (`GameplayStatics.GetPlayerCharacter` 0)))
      (set `self.As BP Chara NPC` _asbp_chara_npc)))
  (return (`self.As BP Chara NPC`)))

(fn `UserConstructionScript`)