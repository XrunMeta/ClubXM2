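; Club speaker Blueprint that plays a looping music playlist from BeginPlay.
; Each finished track advances SongID through Songlist, wrapping at the end, with volume read from the GameInstance's saved music setting.
; It also handles the GameInstance's audio-adjust event by restarting the current song, storing SFX, notification and voice-chat volumes on the GameInstance, and having the player controller update voice volume.
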(event `PlaySong 2nd Floor`
  (bind _audiocomponent (`self.AudioComponent`))
  (bind _audiocomponent_2 (`self.AudioComponent`))
  (bind _asbp_game_instance (cast `/Game/Blueprints/Subsystem/BP_GameInstance` (`GameplayStatics.GetGameInstance`) :!label _label))
  (bind _output_get (set `self.As BP Game Instance` _asbp_game_instance))
  (add `/Game/Blueprints/Subsystem/BP_GameInstance.OnAdjustAudio` _output_get (delegate `OnAdjustAudio_Event`))
  ;[1 1 1] Delegates on Begin Play and Play Song for the first time
  (add `AudioComponent.OnAudioPlaybackPercent` _audiocomponent_2 (delegate `OnAudioPlaybackPercent_Event`))
  (add `AudioComponent.OnAudioFinished` _audiocomponent_2 (delegate `OnAudioFinished_Event`))
  ;[1 1 1] Play Song
  (`AudioComponent.SetSound` _audiocomponent (`|GetArrayItem` (`self.Songlist`) (`self.SongID`)) :!label _label_2)
  (`AudioComponent.Play` (`self.AudioComponent`) 0.0)
  (`AudioComponent.AdjustVolume` _audiocomponent 0.0 (`.Audio_Music_8_EFCD063E48F04452BBCE2EA8BE60A70C` (break `/Game/Gamefolder/Rian/S_Settings` (`/Game/Blueprints/Subsystem/BP_GameInstance.SettingsStruct` (`self.As BP Game Instance`)))) "Linear"))

(event `PlaySong`
  (params (Music :type "Float (double-precision)"))
  ;[1 1 1] Play Song
  (goto _label_2))

(event `self.ReceiveBeginPlay`
  (goto _label))

(event `SongFinishedPlaying`
  ;[1 1 1] Song is finished playing, play next song and repeat playlist
  (if (== (`self.SongID`) (`KismetArrayLibrary.Array_LastIndex` (`self.Songlist`)))
    (set `self.SongID` 0)
    (else
      (`/Engine/EditorBlueprintResources/StandardMacros.IncrementInt` (`self.SongID`)
        (:`  `
          _))))
  (`self.PlaySong` (`self.Music`)))

(event `OnAdjustAudio_Event`
  (params (Music :type "Float (double-precision)") (SFX :type "Float (double-precision)") (Notification :type "Float (double-precision)") (VoiceChat :type "Float (double-precision)"))
  (bind _as_bp_game_instance (`self.As BP Game Instance`))
  (bind _output_get (set `self.Music` Music))
  (`self.PlaySong` _output_get)
  (set `/Game/Blueprints/Subsystem/BP_GameInstance.SFX Volume` SFX _as_bp_game_instance)
  (set `/Game/Blueprints/Subsystem/BP_GameInstance.Notification Volume` Notification _as_bp_game_instance)
  (set `/Game/Blueprints/Subsystem/BP_GameInstance.Voice chat Volume` VoiceChat _as_bp_game_instance)
  (`/Game/Blueprints/PlayerController/BP_PlayerController.Control Voice Volume` (cast `/Game/Blueprints/PlayerController/BP_PlayerController` (`GameplayStatics.GetPlayerController` 0) :!pure true)))

(event `OnAudioFinished_Event`
  ;[1 1 1] Delegates on Begin Play and Play Song for the first time
  (`self.SongFinishedPlaying`))

(event `OnAudioPlaybackPercent_Event`
  (params (PlayingSoundWave :type "SoundWave Object Reference") (PlaybackPercent :type "Float (single-precision)"))
  ;[1 1 1] Delegates on Begin Play and Play Song for the first time
)

(fn `UserConstructionScript`)