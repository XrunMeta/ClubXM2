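; VR player controller that switches the local player between headset and flat-screen rendering at BeginPlay.
; With an HMD connected in a game or VR preview session that is not unattended, console commands set full resolution quality and pixel density, force stereo, and enable the HMD.
; Otherwise, after a short delay, it turns stereo and start-in-VR off and disables the HMD.
; Remote controllers skip the setup, and Tick is unused.
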(event `self.ReceiveBeginPlay`
  (`parent.ReceiveBeginPlay`)
  (if (`self.IsLocalController`)
    (if (and (`VRExpansionFunctionLibrary.GetIsHMDConnected`) (not (`KismetSystemLibrary.IsUnattended`)) (`VRExpansionFunctionLibrary.IsInVREditorPreviewOrGame`))
      (`KismetSystemLibrary.ExecuteConsoleCommand` "sg.ResolutionQuality 100" self)
      (`KismetSystemLibrary.ExecuteConsoleCommand` "vr.bEnableStereo true" self) ; Forces stereo here as it hasn't been done yet for server
      (`KismetSystemLibrary.ExecuteConsoleCommand` "r.screenpercentage 100" null)
      (`KismetSystemLibrary.ExecuteConsoleCommand` "vr.PixelDensity 1" null)
      (`KismetSystemLibrary.ExecuteConsoleCommand` "vr.bStartInVR 1" null)
      (`HeadMountedDisplayFunctionLibrary.EnableHMD` true)
      (else
        (`KismetSystemLibrary.Delay` 0.2) ; Delay for proper tracking data, could also loop\nuntil it returns valid with a max loop count.
        (`KismetSystemLibrary.ExecuteConsoleCommand` "vr.bEnableStereo false" self) ; Oculus Only
        (`KismetSystemLibrary.ExecuteConsoleCommand` "vr.bStartInVR 0" null)
        (`HeadMountedDisplayFunctionLibrary.EnableHMD` false)))))

(fn `UserConstructionScript`
  (`parent.UserConstructionScript`))