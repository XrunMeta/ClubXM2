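; Moving hazard actor in the population system that oscillates along world X and ragdolls pawns it touches.
; From BeginPlay, StartMove computes a target Offset units away, and a Timeline lerps the actor there without sweep.
; A FlipFlop on each Timeline finish restarts the move in the opposite direction, looping indefinitely.
; Sphere1 overlaps with a BP_BasePawn call its EnableRagdoll.
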(event `self.ReceiveBeginPlay`
  (`self.StartMove` true))

(event `StartMove`
  (params (Forward :type Boolean))
  (set `self.CurrentLocation` (`self.K2_GetActorLocation`))
  (set `self.TargetLocation` (`KismetMathLibrary.MakeVector` (+ (.x (`self.CurrentLocation`)) (* (`self.Offset`) (`KismetMathLibrary.SelectFloat` 1.0 -1.0 Forward))) (.y (`self.CurrentLocation`)) (.z (`self.CurrentLocation`))))
  (bind (_direction _alpha) (`Timeline|Timeline_0` :!via `PlayFromStart`)
    (:`Update`
      (`self.K2_SetActorLocation` (`KismetMathLibrary.VLerp` (`self.CurrentLocation`) (`self.TargetLocation`) _alpha)))
    (:`Finished`
      (`/Engine/EditorBlueprintResources/StandardMacros.FlipFlop`
        (:`A`
          (`self.StartMove` false))
        (:`B`
          (`self.StartMove` true))))))

(event `self.Sphere1.OnComponentBeginOverlap`
  (params (OverlappedComponent :type "PrimitiveComponent Object Reference") (OtherActor :type "Actor Object Reference") (OtherComp :type "PrimitiveComponent Object Reference") (OtherBodyIndex :type Integer) (bFromSweep :type Boolean) (SweepResult :type "HitResult Structure (by ref)"))
  (bind _asbp_base_pawn (cast `/Game/Population_System/Blueprints/BP_BasePawn` OtherActor))
  (`/Game/Population_System/Blueprints/BP_BasePawn.EnableRagdoll` _asbp_base_pawn))

(fn `UserConstructionScript`)