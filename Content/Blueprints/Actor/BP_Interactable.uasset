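; Interactable actor that registers itself with the player character while the player stands inside its Box trigger.
; On begin overlap it caches the BP_PlayerCharacter, passes itself through InteractableActorMessage and shows the interactable indicator on the player's gameplay HUD.
; On end overlap it sends the same message with no actor and hides the indicator.
; It holds no interaction behavior of its own.
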(event `self.ReceiveBeginPlay`)

(event `self.Box.OnComponentBeginOverlap`
  (params (OverlappedComponent :type "PrimitiveComponent Object Reference") (OtherActor :type "Actor Object Reference") (OtherComp :type "PrimitiveComponent Object Reference") (OtherBodyIndex :type Integer) (bFromSweep :type Boolean) (SweepResult :type "HitResult Structure (by ref)"))
  (bind _asbp_player_character (cast `/Game/Blueprints/Character/BP_PlayerCharacter` OtherActor))
  (bind _output_get (set `self.As BP Player Character` _asbp_player_character))
  (`/Engine/EditorBlueprintResources/StandardMacros.IsValid` _output_get
    (:`Is Valid`
      (if (== _output_get OtherActor)
        (message `/Game/Blueprints/Interface/BPI_InteractionInterface.InteractableActor` OtherActor self)
        (bind _as_bp_gameplay_hud (`/Game/Blueprints/Character/BP_PlayerCharacter.As BP Gameplay HUD` (`self.As BP Player Character`))
          (:`then`
            (`/Game/Blueprints/HUD/BP_GameplayHUD.SetInteractableVisibility` _as_bp_gameplay_hud true))
          (:`else`))))))

(event `self.Box.OnComponentEndOverlap`
  (params (OverlappedComponent :type "PrimitiveComponent Object Reference") (OtherActor :type "Actor Object Reference") (OtherComp :type "PrimitiveComponent Object Reference") (OtherBodyIndex :type Integer))
  (bind _as_bp_player_character (`self.As BP Player Character`))
  (`/Engine/EditorBlueprintResources/StandardMacros.IsValid` _as_bp_player_character
    (:`Is Valid`
      (if (== OtherActor _as_bp_player_character)
        (message `/Game/Blueprints/Interface/BPI_InteractionInterface.InteractableActor` _as_bp_player_character null)
        (bind _as_bp_gameplay_hud (`/Game/Blueprints/Character/BP_PlayerCharacter.As BP Gameplay HUD` _as_bp_player_character)
          (:`then`
            (`/Game/Blueprints/HUD/BP_GameplayHUD.SetInteractableVisibility` _as_bp_gameplay_hud false))
          (:`else`))))))

(fn `UserConstructionScript`)