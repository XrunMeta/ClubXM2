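; Multiplayer player character with character selection, name tag, chat and friend-list hotkeys, and radial quick-tool and build menus.
; SR_ events handle mesh choice and movement locking, while RepNotifies apply the mesh and name tag text.
; Menu events swap input modes; build mode also slows time but only prints the committed item, and some old menu wiring is disconnected.
; Tick copies CameraBoom's target roll and yaw onto a second spring arm.
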(event `self.ReceiveBeginPlay`
  (`parent.ReceiveBeginPlay`))

(event `RadialMenu`
  ;[0 0.2945 1] Radial Menu
  (`self.EnterQuickItem`))

(event `EnterQuickItem`
  ;[0 0.85 1 1 36] Inventory
  (`self.builder_menu`
    (:`then`)
    (:`else`
      ;;[0.01562 0.01562 0.01562] Standard way of adding a widget to the screen
      (bind _returnvalue (`|CreateWidget` "/Game/GenericRadialMenus/Example/InventorySample/UMG_TestInventoryMenu.UMG_TestInventoryMenu_C" (`GameplayStatics.GetPlayerController` 0)))
      (bind _output_get (set `self.ItemSelector` _returnvalue))
      (`UserWidget.AddToViewport` _output_get 0)
      ;;[0.5421 0 0.8542 1 24] IMPORTANT NOTE: to allow joystick input into the Radial menu, the controller must be in "Game" mode or "Game and UI". "UI Only" mode does not seem to allow access to the joystick input.
      (`WidgetBlueprintLibrary.SetInputMode_GameAndUIEx` (`GameplayStatics.GetPlayerController` 0) (`self.ItemSelector`) "LockAlways")
      (`Controller.SetIgnoreLookInput` (`GameplayStatics.GetPlayerController` 0) true))))

(event `Key|LeftShift`
  (params (Key :type "Key Structure"))
  ;[0 0.2945 1] Radial Menu
)

(event `self.ReceiveTick`
  (params (DeltaSeconds :type "Float (single-precision)"))
  (bind (_returnvalue_roll _returnvalue_pitch _returnvalue_yaw) (`KismetMathLibrary.BreakRotator` (`SpringArmComponent.GetTargetRotation` (`self.CameraBoom`))))
  (bind (_returnvalue_roll_2 _returnvalue_pitch_2) (`KismetMathLibrary.BreakRotator` (`SpringArmComponent.GetTargetRotation` (`self.SpringArm_0`))))
  (`parent.ReceiveTick` DeltaSeconds)
  (`SceneComponent.K2_SetRelativeRotation` (`self.SpringArm_0`) (`KismetMathLibrary.MakeRotator` _returnvalue_roll _returnvalue_pitch_2 _returnvalue_yaw) false false))

(event `ExitQuickItem`
  (bind (_outindex _valid) (`/Game/GenericRadialMenus/Example/InventorySample/UMG_TestInventoryMenu.GetSelectedOption` (`self.ItemSelector`)))
  ;[0 0.85 1 1 36] Inventory
  (bind _itemselector (`self.ItemSelector`)
    (:`then`
      (`Widget.RemoveFromParent` _itemselector)
      (`WidgetBlueprintLibrary.SetInputMode_GameOnly` (`GameplayStatics.GetPlayerController` 0))
      (`Controller.SetIgnoreLookInput` (`GameplayStatics.GetPlayerController` 0) false)
      (if _valid
        (set `self.ChosenTool` _outindex)
        (`GameplayStatics.PlaySound2D` "/Engine/VREditor/Sounds/UI/Dockable_Window_Open.Dockable_Window_Open" 1.0 1.0 0.0 null null))
      (set `self.ItemSelector` null))
    (:`else`)))

(event `SubmenuCommited`
  (params (Category :type Name) (SubItem :type Name))
  ;[0 0.85 1 1 36] Build Menu
  ;;[0.6094 0 0] This is called when a build item has been chosen.
  (`KismetSystemLibrary.PrintString` (`KismetStringLibrary.Concat_StrStr` "Build " (`KismetStringLibrary.Conv_NameToString` SubItem) " " (`KismetStringLibrary.Conv_NameToString` Category))))

(event `EnterBuildMode`
  ;[0 0.85 1 1 36] Build Menu
  (`self.ItemSelector`
    (:`then`)
    (:`else`
      (bind _returnvalue (`|CreateWidget` "/Game/GenericRadialMenus/Templates/UMG_MultiMenuTemplate.UMG_MultiMenuTemplate_C"))
      (bind _output_get (set `self.builder_menu` _returnvalue))
      (`UserWidget.AddToViewport` _output_get 0)
      (`GameplayStatics.SetGlobalTimeDilation` 0.1)
      ;;[0.5421 0 0.8542 1 24] IMPORTANT NOTE: to allow joystick input into the Radial menu, the controller must be in "Game" mode or "Game and UI". "UI Only" mode does not seem to allow access to the joystick input.
      (`WidgetBlueprintLibrary.SetInputMode_GameAndUIEx` (`GameplayStatics.GetPlayerController` 0) (`self.builder_menu`) "LockAlways")
      (`self.DisableInput` (`GameplayStatics.GetPlayerController` 0))
      (add `/Game/GenericRadialMenus/Templates/UMG_SimpleInputWidget.Cancel` (`self.builder_menu`) (delegate `ExitBuild`))
      (add `/Game/GenericRadialMenus/Templates/UMG_SimpleInputWidget.SubmenuCommit` (`self.builder_menu`) (delegate `SubmenuCommited`)))))

(event `ExitBuild`
  ;[0 0.85 1 1 36] Build Menu
  (`self.ItemSelector`
    (:`then`)
    (:`else`
      (bind _builder_menu (`self.builder_menu`)
        (:`then`
          (`Widget.RemoveFromParent` _builder_menu)
          (`GameplayStatics.SetGlobalTimeDilation` 1.0)
          (`WidgetBlueprintLibrary.SetInputMode_GameOnly` (`GameplayStatics.GetPlayerController` 0))
          (`GameplayStatics.PlaySound2D` "/Engine/VREditor/Sounds/UI/Dockable_Window_Open.Dockable_Window_Open" 1.0 1.0 0.0 null null)
          (set `self.builder_menu` null)
          (`self.EnableInput` (`GameplayStatics.GetPlayerController` 0)))
        (:`else`)))))

(event `SR_RepChangeMesh`
  (params (`Selected Skeletal Mesh` :type "SkeletalMesh Object Reference"))
  ;[1 1 1] Change Skeletal Mesh RepNotify
  (set `self.SelectedMesh_0` `Selected Skeletal Mesh`)
  (`CharacterMovementComponent.SetMovementMode` (`self.CharacterMovement`) "MOVE_Walking" 0))

(event `self.BPIF_ApplyCharacterSelect`
  (params (Selected_Skeletalmesh :type "SkeletalMesh Object Reference"))
  ;[1 1 1] Change Skeletal Mesh RepNotify
  (`self.SR_RepChangeMesh` Selected_Skeletalmesh))

(event `self.BPIF_CancelCharacterSelect`
  (params (`Current Mesh` :type "SkeletalMesh Object Reference"))
  ;[1 1 1] Cancel Change Player
  (`SkeletalMeshComponent.SetSkeletalMeshAsset` (`self.Mesh`) `Current Mesh`))

(event `SR_DisableMovement`
  ;[1 1 1] Set Character movement when choosing character
  (`CharacterMovementComponent.DisableMovement` (`self.CharacterMovement`)))

(event `self.BPIF_SetMovementPlayer`
  (params (`DisableMovement?` :type Boolean))
  ;[1 1 1] Set Character movement when choosing character
  (if `DisableMovement?`
    (`self.SR_DisableMovement`)
    (else
      (`self.SR_SetMovementWalking`))))

(event `SR_SetMovementWalking`
  ;[1 1 1] Set Character movement when choosing character
  (`CharacterMovementComponent.SetMovementMode` (`self.CharacterMovement`) "MOVE_Walking" 0))

(event `Key|LeftControl`
  (params (Key :type "Key Structure"))
  ;[1 1 1] show cursor
  (:`Pressed`
    (set `PlayerController.bShowMouseCursor` (not (`PlayerController.bShowMouseCursor` (`GameplayStatics.GetPlayerController` 0))) (`GameplayStatics.GetPlayerController` 0))
    (if (`PlayerController.bShowMouseCursor` (`GameplayStatics.GetPlayerController` 0))
      (`WidgetBlueprintLibrary.SetInputMode_GameAndUIEx` (`GameplayStatics.GetPlayerController` 0) null "LockAlways")
      (else
        (`WidgetBlueprintLibrary.SetInputMode_GameOnly` (`GameplayStatics.GetPlayerController` 0))))))

(event `Key|Enter`
  (params (Key :type "Key Structure"))
  ;[1 1 1] show chat
  (:`Released`
    (bind _chatac (`self.INFRefChatAC`))
    (`/Game/MultiplayerChatSys/Blueprint/Component/Chat_AC.FuncShowChat` _chatac true)))

(event `Key|F`
  (params (Key :type "Key Structure"))
  ;[1 1 1] show friend list
  (:`Pressed`
    (bind _mainwidget (`/Game/MultiplayerChatSys/Blueprint/Interfaces/BPI_ChatterCharacter.INFRefMainWidgetChatter`))
    (`/Game/MultiplayerChatSys/Blueprint/HUD/PlayerList/PlayerListContainer_Widget.CustEvent_ShowOrHidePlayerList` (`/Game/MultiplayerChatSys/Blueprint/HUD/_Main_Widget.PlayerListContainer_Widget` _mainwidget))))

(event `self.INFUpdateNameTagsWidget`
  (params (PlayerName :type String))
  ;[1 1 1] set player name
  (set `self.PlayerName` PlayerName))

(fn `GetCurrentTool`
  (returns (Output :type "/Game/GenericRadialMenus/Example/InventorySample/ToolData Structure"))
  (return (`|GetArrayItem` (`self.Tools`) (`self.ChosenTool`))))

(fn `INFGetPlayerNameChatter`
  (returns (PlayerName :type String))
  (return (`self.PlayerName`)))

(fn `INFRefChatAC`
  (returns (ChatAC :type "/Game/MultiplayerChatSys/Blueprint/Component/Chat_AC Object Reference"))
  (return (`self.Chat_AC`)))

(fn `INFRefChatContainer`
  (returns (ChatContainerWidget :type "/Game/MultiplayerChatSys/Blueprint/HUD/Chat/ChatContainer_Widget Object Reference"))
  (bind _mainwidget (`self.INFRefMainWidgetChatter`))
  (return (`/Game/MultiplayerChatSys/Blueprint/HUD/_Main_Widget.ChatContainer_Widget` _mainwidget)))

(fn `INFRefGameChatterAC`
  (returns (GameChatterAC :type "/Game/MultiplayerChatSys/Blueprint/Component/GameChatter_AC Object Reference"))
  (bind _gamechatterac (message `/Game/MultiplayerChatSys/Blueprint/Interfaces/BPI_ChatterGameMode.INFRefGameChatterAC` (`GameplayStatics.GetGameMode`)))
  (return _gamechatterac))

(fn `INFRefMainWidgetChatter`
  (returns (MainWidget :type "/Game/MultiplayerChatSys/Blueprint/HUD/_Main_Widget Object Reference"))
  (bind _chatac (`self.INFRefChatAC`))
  (return (`/Game/MultiplayerChatSys/Blueprint/Component/Chat_AC.MainWidget` _chatac)))

(fn `OnRep_PlayerName`
  (if (not (`KismetSystemLibrary.IsDedicatedServer`))
    (bind _asnames_tag_widget (cast `/Game/MultiplayerChatSys/Blueprint/HUD/NamesTag_Widget` (`WidgetComponent.GetUserWidgetObject` (`self.NameTagsWidget`))))
    (`/Game/MultiplayerChatSys/Blueprint/HUD/NamesTag_Widget.FuncUpdateNames` _asnames_tag_widget (`self.PlayerName`))))

(fn `OnRep_SelectedMesh`
  (`SkeletalMeshComponent.SetSkeletalMeshAsset` (`self.Mesh`) (`self.SelectedMesh_0`)))

(fn `UserConstructionScript`
  (`parent.UserConstructionScript`))