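; BP_LobbyHUD is the lobby HUD that detects VR on BeginPlay and otherwise runs the startup screen sequence.
; With an active headset, it only sets IsVR on BP_GameInstance.
; Otherwise it locks portrait orientation, then shows the Bink intro and loading screen widgets on fixed delays before adding the WBP_Login_FIXED login widget.
; An alternative ClubX opening intro branch is left disconnected.
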(event `self.ReceiveBeginPlay`
  ;[1 0 0] Unplug for Mobile packaging
  (if (and (`VRExpansionFunctionLibrary.GetIsHMDConnected`) (not (`KismetSystemLibrary.IsUnattended`)) (`VRExpansionFunctionLibrary.IsInVREditorPreviewOrGame`))
    (bind _asbp_game_instance (cast `/Game/Blueprints/Subsystem/BP_GameInstance` (`GameplayStatics.GetGameInstance`)))
    (set `/Game/Blueprints/Subsystem/BP_GameInstance.IsVR` true _asbp_game_instance)
    (else
      (`BlueprintPlatformLibrary.SetAllowedDeviceOrientation` "Portrait")
      ;[1 1 1] Bink Intro Vertical
      (bind _returnvalue (`|CreateWidget` "/Game/Widget/Login_Register/WBP_IntroBink.WBP_IntroBink_C" (`self.GetOwningPlayerController`)))
      (`UserWidget.AddToViewport` _returnvalue 0)
      (`KismetSystemLibrary.Delay` 5.0)
      (`Widget.RemoveFromParent` _returnvalue)
      ;[1 1 1] Play Loading Screen Video
      (bind _returnvalue_2 (`|CreateWidget` "/Game/Widget/Login_Register/WBP_LoadingScreen.WBP_LoadingScreen_C" (`self.GetOwningPlayerController`)))
      (`UserWidget.AddToViewport` _returnvalue_2 0)
      (`KismetSystemLibrary.Delay` 5.0)
      (`Widget.RemoveFromParent` _returnvalue_2)
      (bind _returnvalue_3 (`|CreateWidget` "/Game/Blueprints/Widgets/WBP_Login_FIXED.WBP_Login_FIXED_C" (`self.GetOwningPlayerController`)))
      (`UserWidget.AddToViewport` _returnvalue_3 0))))

(fn `UserConstructionScript`)