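; Animated club disco light Blueprint with a strobing yellow beam.
; BeginPlay scales the beam static mesh, snaps it to the skeletal mesh's SocketBeam socket and loops a light animation at a configurable play rate.
; A fast looping timer fires Kedip2, which uses a FlipFlop to switch DiffusePower on and off.
; Each tick of that timer creates a new dynamic material instance on the beam to apply the power and yellow color.
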(event `self.ReceiveBeginPlay`
  (bind _staticmesh (`self.StaticMesh`))
  (`SceneComponent.SetRelativeScale3D` _staticmesh (1.25 4.8 1.25))
  (`SceneComponent.K2_AttachToComponent` _staticmesh (`self.SkeletalMeshComponent`) "SocketBeam" "SnapToTarget" "KeepRelative" "KeepRelative" true)
  (`SkeletalMeshComponent.PlayAnimation` (`self.SkeletalMeshComponent`) "/Game/Club_Assets/SHARED/StageEquipment/Animations/Anim_DiscoLight04_2.Anim_DiscoLight04_2" true)
  (`SkeletalMeshComponent.SetPlayRate` (`self.SkeletalMeshComponent`) (`self.PlayRate`))
  (`KismetSystemLibrary.K2_SetTimerDelegate` (delegate `Kedip2`) 0.08 true))

(event `Kedip2`
  (`/Engine/EditorBlueprintResources/StandardMacros.FlipFlop`
    (:`A`
      (set `self.DiffusePower` 5.0))
    (:`B`
      (set `self.DiffusePower` 0.0)))
  (bind _returnvalue (`PrimitiveComponent.CreateDynamicMaterialInstance` (`self.StaticMesh`) 0 "/Game/Club_Assets/SHARED/StageEquipment/Materials/M_LightBeamyellow.M_LightBeamyellow" "None"))
  (`MaterialInstanceDynamic.SetScalarParameterValue` _returnvalue "DiffusePower" (`self.DiffusePower`))
  (`MaterialInstanceDynamic.SetVectorParameterValue` _returnvalue "Color" (make `LinearColor` 0.6 0.4 0.05 1.0)))

(fn `UserConstructionScript`)