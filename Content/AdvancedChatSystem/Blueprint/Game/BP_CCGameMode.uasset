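; BP_CCGameMode is the chat system's game mode, tracking connected BP_ChatPlayerControllers and keeping their player lists updated.
; On login it adds the controller, names it from PlayerNames using its array index, then calls SetEntryPlayers on every controller with that name and the receiving controller's own reference.
; On logout it removes the controller and tells remaining controllers to delete that player from their messages list.
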(event `self.K2_PostLogin`
  (params (NewPlayer :type "PlayerController Object Reference"))
  (bind _asbp_chat_player_controller (cast `/Game/AdvancedChatSystem/Blueprint/Game/BP_ChatPlayerController` NewPlayer))
  (bind _returnvalue (`KismetArrayLibrary.Array_Add` (`self.ConnectedPlayers`) _asbp_chat_player_controller))
  (bind _output (`|GetArrayItem` (`self.PlayerNames`) _returnvalue))
  (`/Game/AdvancedChatSystem/Blueprint/Game/BP_ChatPlayerController.SetPlayerName` _asbp_chat_player_controller _output)
  (for _array_element (`self.ConnectedPlayers`)
    (`/Game/AdvancedChatSystem/Blueprint/Game/BP_ChatPlayerController.SetEntryPlayers` _array_element _output _array_element null)))

(event `self.K2_OnLogout`
  (params (ExitingController :type "Controller Object Reference"))
  (bind _asbp_chat_player_controller (cast `/Game/AdvancedChatSystem/Blueprint/Game/BP_ChatPlayerController` ExitingController))
  (bind _returnvalue (`KismetArrayLibrary.Array_RemoveItem` (`self.ConnectedPlayers`) _asbp_chat_player_controller))
  (if _returnvalue
    (for _array_element (`self.ConnectedPlayers`)
      (`/Game/AdvancedChatSystem/Blueprint/Game/BP_ChatPlayerController.DeletePlayerFromMessagesList(Client)` _array_element (`/Game/AdvancedChatSystem/Blueprint/Game/BP_ChatPlayerController.PlayerName` _asbp_chat_player_controller)))))

(fn `UserConstructionScript`)