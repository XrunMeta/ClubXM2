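; Showcase actor for the Minimalist UI Pack that previews a widget in 3D, with a text label set from PreviewText in the Construction Script.
; When ShowOnScreenPreview is enabled, overlapping the Box hides the 3D widget, adds a new instance of its class to the viewport and enables cursor and UI input.
; Leaving removes that instance, restores the 3D widget and game-only input, and resets the DoOnce guard.
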(event `self.Box.OnComponentBeginOverlap`
  (params (OverlappedComponent :type "PrimitiveComponent Object Reference") (OtherActor :type "Actor Object Reference") (OtherComp :type "PrimitiveComponent Object Reference") (OtherBodyIndex :type Integer) (bFromSweep :type Boolean) (SweepResult :type "HitResult Structure (by ref)"))
  (bind _returnvalue (`GameplayStatics.GetPlayerController` 0))
  ;[1 1 1] Add Widget to the Screen when the player overlaps the Box and set the Visibility of the 3D widget to Hidden
  (if (`self.ShowOnScreenPreview`)
    (`/Engine/EditorBlueprintResources/StandardMacros.DoOnce` false :!label _label
      (:`Completed`
        (`SceneComponent.SetVisibility` (`self.Widget`) false false)
        (bind _returnvalue_2 (`|CreateWidget` (`GameplayStatics.GetObjectClass` (`WidgetComponent.GetUserWidgetObject` (`self.Widget`))) _returnvalue))
        (bind _output_get (set `self.CurrentWidget` _returnvalue_2))
        (`UserWidget.AddToViewport` _output_get 0)
        (set `PlayerController.bShowMouseCursor` true _returnvalue)
        (`WidgetBlueprintLibrary.SetInputMode_GameAndUIEx` _returnvalue (`self.CurrentWidget`) "DoNotLock" false)))))

(event `self.Box.OnComponentEndOverlap`
  (params (OverlappedComponent :type "PrimitiveComponent Object Reference") (OtherActor :type "Actor Object Reference") (OtherComp :type "PrimitiveComponent Object Reference") (OtherBodyIndex :type Integer))
  (bind _returnvalue (`GameplayStatics.GetPlayerController` 0))
  ;[1 1 1] Remove the Widget from the Screen when the player leaves the Box, also set the Visiblity of the 3D widget back to Visible
  (if (`self.ShowOnScreenPreview`)
    (`WidgetBlueprintLibrary.SetInputMode_GameOnly` _returnvalue)
    (set `PlayerController.bShowMouseCursor` false _returnvalue)
    (`SceneComponent.SetVisibility` (`self.Widget`) true false)
    (`Widget.RemoveFromParent` (`self.CurrentWidget`))
    (goto _label :!via `Reset`)))

(fn `UserConstructionScript`
  ;[1 1 1] Set the Text of the Text Render
  (`TextRenderComponent.K2_SetText` (`self.TextPreview`) (`self.Preview Text`)))