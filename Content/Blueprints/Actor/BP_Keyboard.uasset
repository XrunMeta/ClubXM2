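; BP_Keyboard is an actor that hosts a virtual keyboard through a widget component.
; On BeginPlay it gets the component's WBP_VirtualKeyboard and hands it a WidgetInteraction reference; no key handling happens in this graph.
; A disconnected leftover fragment casts a TargetDisplay's widget to WBP_InputTextBox and never runs.
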(event `self.ReceiveBeginPlay`
  (bind _aswbp_virtual_keyboard (cast `/Game/Blueprints/Widgets/WBP_VirtualKeyboard` (`WidgetComponent.GetUserWidgetObject` (`self.Widget`))))
  (set `/Game/Blueprints/Widgets/WBP_VirtualKeyboard.WidgetInteraction` (`self.WidgetInteraction`) _aswbp_virtual_keyboard))

(fn `UserConstructionScript`)