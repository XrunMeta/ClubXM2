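; Player controller for the chat system that creates the HUD, toggles the mouse cursor and holds player name and team ID.
; Global and private messages go out through BPChatComponent's server calls, while update events push log entries to the HUD.
; A client-to-server request builds the private-chat player list from the GameMode's connected players, with Steam or default thumbnails.
; Debug keys print the name and set a test team.
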(event Custom|UpdatePlayerChatLog
  (params (PlayerName :type String) (Message :type String) (MessageType :type E_MessageType%20Enum :default "NewEnumerator0") (TargetPlayerName :type String))
  ;[1 1 1] Private messaging
  ;;[1 1 1] Process Player Chats
  (Default|UpdatePlayerChatLog (Variables|Widgets|GetHud) (Utilities|Struct|MakeChatLogEntryStruct PlayerName Message MessageType) TargetPlayerName))

(event Custom|SetEntryPlayers
  (params (PlayerName :type String) (PlayerControllerRef :type BP%20Chat%20Player%20Controller%20Object%20Reference) (Thumbnail :type Texture%202D%20Object%20Reference))
  ;[1 1 1] Private messaging
  ;;[1 1 1] Call up list of players in game
  (bind _wbp_chat_players_box (Variables|Widgets|GetWBP%20Chat%20Players%20Box)
    (:then
      (bind _returnvalue (UserInterface|CreateWidget "/Game/AdvancedChatSystem/Blueprint/UI/WBP_ChatPlayerEntry.WBP_ChatPlayerEntry_C" 0 PlayerName PlayerControllerRef Thumbnail))
      (Widget|Panel|AddChild (Variables|/Game/AdvancedChatSystem/Blueprint/UI/WBP_ChatPlayersBox.WBP_ChatPlayersBox_C|GetEntryBoxScroll _wbp_chat_players_box) _returnvalue))
    (:else)))

(event Custom|CallIUpListOfPlayersInGame%28Client%29
  (params (WBP_ChatPlayersBox :type WBP%20Chat%20Players%20Box%20Object%20Reference))
  ;[1 1 1] Private messaging
  ;;[1 1 1] Call up list of players in game
  (bind _output_get (Variables|Widgets|SetWBP%20Chat%20Players%20Box WBP_ChatPlayersBox))
  (CallFunction|CallIUpListOfPlayersinGame(Server) _output_get))

(event Custom|CallIUpListOfPlayersInGame%28Server%29
  (params (WBP_ChatPlayersBox :type WBP%20Chat%20Players%20Box%20Object%20Reference))
  ;[1 1 1] Private messaging
  ;;[1 1 1] Call up list of players in game
  (CallFunction|CallIUpListOfPlayersinGame WBP_ChatPlayersBox))

(event Custom|SendGlobalChatMessage%28Client%29
  (params (TextToSend :type String) (Message%20Type :type E_MessageType%20Enum :default "NewEnumerator0"))
  ;[1 1 1] Process Global Chats
  (Default|SendGlobalChatMessage(Server) (Variables|Default|GetBP_ChatComponent) (Variables|Default|GetPlayerName) TextToSend self Message%20Type (Variables|Default|GetTeamID)))

(event Custom|UpdateChatLog
  (params (PlayerName :type String) (Message :type String) (MessageType :type E_MessageType%20Enum :default "NewEnumerator0"))
  ;[1 1 1] Process Global Chats
  (Default|UpdateChatLog (Variables|Widgets|GetHud) (Utilities|Struct|MakeChatLogEntryStruct PlayerName Message MessageType)))

(event Custom|DeletePlayerFromMessagesList%28Client%29
  (params (PlayerName :type String))
  ;[1 1 1] Private messaging
  ;;[1 1 1] Delete player from Messages list
  (Default|RemovePlayerChatsInteract (Variables|Widgets|GetHud) PlayerName))

(event Custom|InitializeHUD
  ;[1 1 1] Create hud
  (bind _returnvalue (UserInterface|CreateWidget "/Game/AdvancedChatSystem/Blueprint/UI/WBP_HUD.WBP_HUD_C" self))
  (bind _output_get (Variables|Widgets|SetHud _returnvalue))
  (UserInterface|Viewport|AddtoViewport _output_get 0))

(event Custom|SendPlayerChatMessage%28Client%29
  (params (TextToSend :type String) (TargetPlayerName :type String))
  ;[1 1 1] Private messaging
  ;;[1 1 1] Process Player Chats
  (Default|SendPlayerChatMessage(Server) (Variables|Default|GetBP_ChatComponent) (Variables|Default|GetPlayerName) TextToSend self TargetPlayerName))

(event Custom|SetPlayerName
  (params (NewName :type String))
  ;[1 1 1] Set player name
  (Variables|Default|SetPlayerName NewName))

(event Custom|UpdateTeamID
  ;[1 0 0] This code has been added to test messaging among team members in the messaging system.
  (Variables|Default|SetTeamID "2"))

(event EventBeginPlay
  ;[1 1 1] Create hud
  (CallFunction|InitializeHUD))

(event Input|KeyboardEvents|DebugKeyK
  (params (Key :type Key%20Structure :default "None") (ActionValue :type Input%20Action%20Value%20Structure))
  ;[1 0 0] Player name controll
)

(event Input|KeyboardEvents|DebugKeyK
  (params (Key :type Key%20Structure :default "None") (ActionValue :type Input%20Action%20Value%20Structure))
  ;[1 1 1] PlayerNameDebug
  (:Pressed
    (Development|PrintString (Variables|Default|GetPlayerName))))

(event Input|KeyboardEvents|Enter
  (params (Key :type Key%20Structure :default "None"))
  ;[1 0 0] Show Mouse Cursor
)

(event Input|KeyboardEvents|T
  (params (Key :type Key%20Structure :default "None"))
  ;[1 0 0] Add Team ID
)

(event Input|KeyboardEvents|T
  (params (Key :type Key%20Structure :default "None"))
  ;[1 0 0] This code has been added to test messaging among team members in the messaging system.
  (:Pressed
    (CallFunction|UpdateTeamID)
    (Development|PrintString "Team ID Introduced")))

(event Input|KeyboardEvents|Enter
  (params (Key :type Key%20Structure :default "None"))
  (bind _self self)
  ;[1 1 1] Show Mouse
  (:Pressed
    (bind _output_get (Variables|Default|SetbShowMouseCursor (not (Variables|Default|GetbShowMouseCursor))))
    (if _output_get
      (Input|SetInputModeGameandUI _self 0 "DoNotLock" true false)
      (else
        (Input|SetInputModeGameOnly _self false)))))

(fn ConstructionScript)

(fn CallIUpListOfPlayersinGame
  (params (WBP_ChatPlayersBox :type WBP%20Chat%20Players%20Box%20Object%20Reference))
  (bind _asbp_ccgame_mode (Utilities|Casting|CastToBP_CCGameMode (Game|GetGameMode)))
  (for _array_element (Variables|/Game/AdvancedChatSystem/Blueprint/Game/BP_CCGameMode.BP_CCGameMode_C|GetConnectedPlayers _asbp_ccgame_mode)
    (if (!= _array_element self)
      (CallFunction|SetEntryPlayers (.Return%20PlayerName (CallFunction|GetThumbnailFriends (Variables|BP_ChatPlayerController_C|GetPlayerName _array_element))) _array_element (.Return%20Thumbnail (CallFunction|GetThumbnailFriends (Variables|BP_ChatPlayerController_C|GetPlayerName _array_element)))))))

(fn GetThumbnailFriends
  (params (Player%20Name :type String))
  (for _array_element (Variables|/Script/Engine.GameStateBase|GetPlayerArray (Game|GetGameState))
    (if (Utilities|Enum|Equal(Enum) Player%20Name (.PlayerName (Utilities|Struct|BreakS_PlayerData (Variables|/Game/Blueprints/PlayerState/BP_PlayerState.BP_PlayerState_C|GetPlayerDataStruct (.AsBP%20Player%20State (Utilities|Casting|CastToBP_PlayerState _array_element))))))
      _
      (elif (Variables|/Game/Blueprints/PlayerState/BP_PlayerState.BP_PlayerState_C|GetPlayerSteam (.AsBP%20Player%20State (Utilities|Casting|CastToBP_PlayerState _array_element)))
        _
        (else
          _)))
    (return Player%20Name (select (Variables|/Game/Blueprints/PlayerState/BP_PlayerState.BP_PlayerState_C|GetPlayerSteam (.AsBP%20Player%20State (Utilities|Casting|CastToBP_PlayerState _array_element))) (Variables|/Game/Blueprints/PlayerState/BP_PlayerState.BP_PlayerState_C|GetThumbnail%20Steam%20Player (.AsBP%20Player%20State (Utilities|Casting|CastToBP_PlayerState _array_element))) "/Game/AdvancedChatSystem/Textures/T_OnlineUser.T_OnlineUser"))))