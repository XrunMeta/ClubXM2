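; Player controller that handles EOS voice chat, text chat and per-player client setup.
; Outside VR, BeginPlay configures platform input, creates the chat HUD outside MainWorld and leaves old voice rooms.
; InitVoice chains connect, login, room token and join callbacks into a level-named room, reporting status to the HUD.
; It also relays names, server tags and chat to the server, and handles push-to-talk, scalability, quit prompt and debug keys.
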(event Custom|UpdatePlayerChatLog
  (params (PlayerName :type String) (Message :type String) (MessageType :type E_MessageType%20Enum :default "NewEnumerator0") (TargetPlayerName :type String))
  ;[1 1 1] Private messaging
  ;;[1 1 1] Process Player Chats
  (Default|UpdatePlayerChatLog (Variables|AdvanceChat|GetHud) (Utilities|Struct|MakeChatLogEntryStruct PlayerName Message MessageType) TargetPlayerName))

(event Custom|EOS%20Leave%20EOS%20Voice%20Room
  (params (bWasSuccess :type Boolean) (Result :type EEVIKResultCodes%20Enum :default "Success"))
  ;[1 1 1] Disconnect Voice when enter new Map
  ;;[1 1 1] Leave All Connected Rooms
  (if bWasSuccess
    (Development|PrintString "Leave")
    (else
      (Development|PrintString "Cannot Leave")))
  (Variables|VoiceChat|SetConnectedToGlobalChat? false)
  (Variables|VoiceChat|SetConnectedToPrivateChat? false)
  (Class|EVIKFunctions|LogoutEOSVoiceChat (Class|EVIKFunctions|LoggedinUser) (delegate Custom|EOS%20LogOut%20From%20EOS%20Voice%20Chat)))

(event Custom|GetRoomToken
  (params (RoomName :type String))
  ;[1 1 1] Get Token for Global EOS Voice Chat and Private Chat
  (bind _output_get (Variables|VoiceChat|SetEOS%20Room%20Name RoomName))
  (Class|EVIKFunctions|EOSRoomToken _output_get (Class|EVIKFunctions|LoggedinUser) "10.0.0.1" (delegate Custom|GetEOSVoiceRoomToken_Result)) ; 10.0.0.1
)

(event Custom|CallIUpListOfPlayersInGame%28Client%29
  (params (WBP_ChatPlayersBox :type WBP%20Chat%20Players%20Box%20Object%20Reference))
  ;[1 1 1] Private messaging
  ;;[1 1 1] Call up list of players in game
  (bind _output_get (Variables|AdvanceChat|SetWBP%20Chat%20Players%20Box WBP_ChatPlayersBox))
  (CallFunction|CallIUpListOfPlayersinGame(Server) _output_get))

(event Custom|Get%20GM
  (bind _asbp_gm_tri (Utilities|Casting|CastToBP_GM_Tri (Game|GetGameMode)))
  (for _array_element (Variables|/Game/Developers/metadevwin003/BP_GM_Tri.BP_GM_Tri_C|GetAll_PC _asbp_gm_tri)
    _))

(event Custom|CallIUpListOfPlayersInGame%28Server%29
  (params (WBP_ChatPlayersBox :type WBP%20Chat%20Players%20Box%20Object%20Reference))
  ;[1 1 1] Private messaging
  ;;[1 1 1] Call up list of players in game
  (CallFunction|CallIUpListOfPlayersinGame WBP_ChatPlayersBox))

(event Custom|JoinEOSVoiceRoom_Result
  (params (bWasSuccess :type Boolean) (Result :type EEVIKResultCodes%20Enum :default "Success"))
  ;[1 1 1] Get Token for Global EOS Voice Chat and Private Chat
  (CallFunction|ROSMICActive bWasSuccess)
  (if bWasSuccess
    (Development|PrintString "Join EOS Voice Room Success" false true "(R=0.000000,G=0.080223,B=1.000000,A=1.000000)" 5.0)
    (CallFunction|FSetWarningChat "Join EOS Voice Room Success")
    (bind _returnvalue (Class|EVIKFunctions|GetAllRooms))
    (for _array_element _returnvalue
      (Development|PrintString _array_element true true "(R=0.343891,G=1.000000,B=0.000000,A=1.000000)" 5.0))
    (Utilities|FlowControl|Delay 0.2)
    (bind _returnvalue_2 (Class|EVIKFunctions|TransmittoSelectedRoom (Variables|VoiceChat|GetEOS%20Room%20Name)))
    (if _returnvalue_2
      (Development|PrintString "Transmit Voice READY" false true "(R=0.000000,G=0.018708,B=1.000000,A=1.000000)" 5.0)
      (CallFunction|FSetWarningChat "Transmit Voice READY")
      (bind _returnvalue_3 (Game|GetCurrentLevelName true))
      (if (Utilities|Enum|Equal(Enum) (Variables|VoiceChat|GetEOS%20Room%20Name) _returnvalue_3)
        (Class|BPIInteractionInterface|BPIFSetVoiceButtonEnabled?(Message) (HUD|GetHUD) true)
        (Variables|VoiceChat|SetConnectedToGlobalChat? true))
      (Default|ToggleWarnaGlobalChat (Variables|/Game/Blueprints/Widgets/WBP_MainWidget.WBP_MainWidget_C|GetWBP_MainMenu (Variables|/Game/Blueprints/HUD/BP_GameplayHUD.BP_GameplayHUD_C|GetBP_MainWidget (.AsBP%20Gameplay%20HUD (Utilities|Casting|CastToBP_GameplayHUD (HUD|GetHUD))))) true)
      (else
        (Development|PrintString "Failed Transmit voice" false)
        (CallFunction|FSetWarningChat "Failed Transmit voice")
        (bind _returnvalue_4 (Game|GetCurrentLevelName true))
        (if (Utilities|Enum|Equal(Enum) (Variables|VoiceChat|GetEOS%20Room%20Name) _returnvalue_4)
          (Class|BPIInteractionInterface|BPIFSetVoiceButtonEnabled?(Message) (HUD|GetHUD) true)
          (Variables|VoiceChat|SetConnectedToGlobalChat? false))))
    (else
      (Development|PrintString "Join EOS Voice Room Failed" false)
      (CallFunction|FSetWarningChat "Join EOS Voice Room Failed")
      (bind _returnvalue_5 (Game|GetCurrentLevelName true))
      (if (Utilities|Enum|Equal(Enum) (Variables|VoiceChat|GetEOS%20Room%20Name) _returnvalue_5)
        (Class|BPIInteractionInterface|BPIFSetVoiceButtonEnabled?(Message) (HUD|GetHUD) true)
        (Variables|VoiceChat|SetConnectedToGlobalChat? true)))))

(event Custom|SendGlobalChatMessage%28Client%29
  (params (TextToSend :type String) (Message%20Type :type E_MessageType%20Enum :default "NewEnumerator0"))
  ;[1 1 1] Process Global Chats
  (Default|SendGlobalChatMessage(Server) (Variables|Default|GetBP_ChatComponent) (Variables|AdvanceChat|GetPlayerName) TextToSend self Message%20Type (Variables|AdvanceChat|GetTeamID)))

(event Custom|EnterServer
  (params (MapIPAddress :type String))
  (Development|ExecuteConsoleCommand MapIPAddress 0))

(event Custom|UpdateChatLog
  (params (PlayerName :type String) (Message :type String) (MessageType :type E_MessageType%20Enum :default "NewEnumerator0"))
  ;[1 1 1] Process Global Chats
  (Default|UpdateChatLog (Variables|AdvanceChat|GetHud) (Utilities|Struct|MakeChatLogEntryStruct PlayerName Message MessageType)))

(event Custom|OC_Ambil_ServerTagGI
  (bind _asbp_gi_club_xtest (Utilities|Casting|CastToBP_GI_ClubXTest (Game|GetGameInstance)))
  (Development|PrintString (Utilities|String|Append "OC_Ambil_ServerTagGI: " (Utilities|String|ToString(Name) (Variables|/Game/Developers/metadevwin003/BP_GI_ClubXTest.BP_GI_ClubXTest_C|GetServerTag _asbp_gi_club_xtest))) false)
  (CallFunction|SRNgasiGI (Variables|/Game/Developers/metadevwin003/BP_GI_ClubXTest.BP_GI_ClubXTest_C|GetServerTag _asbp_gi_club_xtest)))

(event Custom|SetEntryPlayers
  (params (PlayerName :type String) (PlayerControllerRef :type BP%20Player%20Controller%20Object%20Reference))
  ;[1 1 1] Private messaging
  ;;[1 1 1] Call up list of players in game
  (bind _wbp_chat_players_box (Variables|AdvanceChat|GetWBP%20Chat%20Players%20Box)
    (:then
      (bind _returnvalue (UserInterface|CreateWidget "/Game/AdvancedChatSystem/Blueprint/UI/WBP_ChatPlayerEntry.WBP_ChatPlayerEntry_C" 0 PlayerName PlayerControllerRef))
      (Widget|Panel|AddChild (Variables|/Game/AdvancedChatSystem/Blueprint/UI/WBP_ChatPlayersBox.WBP_ChatPlayersBox_C|GetEntryBoxScroll _wbp_chat_players_box) _returnvalue))
    (:else)))

(event Custom|DeletePlayerFromMessagesList%28Client%29
  (params (PlayerName :type String))
  ;[1 1 1] Private messaging
  ;;[1 1 1] Delete player from Messages list
  (Default|RemovePlayerChatsInteract (Variables|AdvanceChat|GetHud) PlayerName))

(event Custom|OC_SetPlayerName
  (bind _asbp_game_instance (Utilities|Casting|CastToBP_GameInstance (Game|GetGameInstance)))
  (CallFunction|SRSetPlayerName (.PlayerName (Utilities|Struct|BreakS_PlayerData (Variables|/Game/Blueprints/Subsystem/BP_GameInstance.BP_GameInstance_C|GetPlayerDataStruct _asbp_game_instance)))))

(event Custom|EOS%20LogOut%20From%20EOS%20Voice%20Chat
  (params (bWasSuccess :type Boolean) (Result :type EEVIKResultCodes%20Enum :default "Success"))
  ;[1 1 1] Disconnect Voice when enter new Map
  ;;[1 1 1] Leave All Connected Rooms
  (if bWasSuccess
    (Development|PrintString "Logged Out")
    (else
      (Development|PrintString "Cannot logout")))
  (Variables|VoiceChat|SetConnectedToGlobalChat? false)
  (Variables|VoiceChat|SetConnectedToPrivateChat? false))

(event Custom|SR_SetPlayerName
  (params (PlayerName :type String))
  (bind _output_get (Variables|AdvanceChat|SetPlayerName PlayerName))
  (bind _asbp_gameplay_game_mode (Utilities|Casting|CastToBP_GameplayGameMode (Game|GetGameMode)))
  (Default|PassPlayerName _asbp_gameplay_game_mode _output_get))

(event Custom|Show%20Die%20Widget
  (bind _returnvalue (UserInterface|CreateWidget "/Game/Blueprints/Widgets/WBP_EnterClubNotif.WBP_EnterClubNotif_C" 0 "You die.. Game will restart"))
  (UserInterface|Viewport|AddtoViewport _returnvalue 0)
  (Utilities|FlowControl|Delay 5.0)
  (Widget|RemovefromParent _returnvalue))

(event Custom|Set%20Volume%20Voice%20Chat
  (bind _eos_username (Variables|VoiceChat|GetEOS%20Username))
  (Class|EVIKFunctions|SetPlayerVolume _eos_username (Variables|/Game/Blueprints/Subsystem/BP_GameInstance.BP_GameInstance_C|GetVoice%20chat%20Volume (Variables|Default|GetAs%20BP%20Game%20Instance)))
  (Development|PrintString (Utilities|String|Append "Volume :   --- " (Utilities|String|ToString(Float) (Class|EVIKFunctions|GetPlayerVolume _eos_username))) true true "(R=0.005281,G=1.000000,B=0.000000,A=1.000000)" 2e+01 "Volume"))

(event Custom|Control%20Voice%20Volume
  (bind _returnvalue (Class|EVIKFunctions|GetPlayersinRoom (Variables|VoiceChat|GetEOS%20Room%20Name)))
  (for _array_element _returnvalue
    (if (not (Utilities|Enum|Equal(Enum) _array_element (Variables|VoiceChat|GetEOS%20Username)))
      (Class|EVIKFunctions|SetPlayerVolume _array_element (Variables|/Game/Blueprints/Subsystem/BP_GameInstance.BP_GameInstance_C|GetVoice%20chat%20Volume (Variables|Default|GetAs%20BP%20Game%20Instance))))))

(event Custom|Show%20Global%20Chat%20from%20shortcut
  (bind _hud (Variables|AdvanceChat|GetHud))
  (bind _globalchatwbp (Variables|/Game/AdvancedChatSystem/Blueprint/UI/WBP_HUD.WBP_HUD_C|GetGlobalChatWbp _hud))
  (Widget|SetVisibility _globalchatwbp (select (Widget|IsVisible _globalchatwbp) "Collapsed" "Visible")))

(event Custom|ROS%20MIC%20Active
  (params (Voice%20Chat%20Active? :type Boolean))
  (Variables|/Game/Blueprints/PlayerState/BP_PlayerState.BP_PlayerState_C|SetVoice%20Chat%20Active? (.AsBP%20Player%20State (Utilities|Casting|CastToBP_PlayerState (Variables|Default|GetPlayerState self))) Voice%20Chat%20Active?))

(event Custom|ROS%20Push%20to%20Talk
  (params (PTT :type Boolean))
  (bind _asbp_player_state (Utilities|Casting|CastToBP_PlayerState (Variables|Default|GetPlayerState self)))
  (bind _output_get (Variables|/Game/Blueprints/PlayerState/BP_PlayerState.BP_PlayerState_C|SetPTT _asbp_player_state PTT))
  (Class|EVIKFunctions|SetPlayerMuted (Variables|VoiceChat|GetEOS%20Username) (not _output_get)))

(event Custom|InitializeHUD
  ;[1 1 1] Create hud on Begin Play
  (bind _returnvalue (Game|GetCurrentLevelName true))
  (if (Utilities|Enum|Equal(Enum) _returnvalue "MainWorld")
    (Widget|SetVisibility (Variables|/Game/AdvancedChatSystem/Blueprint/UI/WBP_HUD.WBP_HUD_C|GetGlobalChatWbp (Variables|AdvanceChat|GetHud)) "Collapsed")
    (else
      (Utilities|IsValid (Variables|AdvanceChat|GetHud)
        (:Is%20Valid
          (Default|RemoveSelffromtheList (Variables|/Game/AdvancedChatSystem/Blueprint/UI/WBP_HUD.WBP_HUD_C|GetWBP_ChatPlayersBox (Variables|AdvanceChat|GetHud))))
        (:Is%20Not%20Valid
          (bind _returnvalue_2 (UserInterface|CreateWidget "/Game/AdvancedChatSystem/Blueprint/UI/WBP_HUD.WBP_HUD_C" self))
          (Variables|AdvanceChat|SetHud _returnvalue_2)))
      (UserInterface|Viewport|AddtoViewport (Variables|AdvanceChat|GetHud) 99)
      (Widget|SetVisibility (Variables|AdvanceChat|GetHud) "Collapsed"))))

(event Custom|GetEOSVoiceRoomToken_Result
  (params (bWasSuccess :type Boolean) (RoomData :type String))
  ;[1 1 1] Get Token for Global EOS Voice Chat and Private Chat
  (if bWasSuccess
    (Development|PrintString "Getting Voice Token")
    (CallFunction|FSetWarningChat "Getting Voice Token")
    (Class|EVIKFunctions|JoinEOSRoom (Variables|VoiceChat|GetEOS%20Room%20Name) RoomData false (delegate Custom|JoinEOSVoiceRoom_Result))
    (else
      (Development|PrintString "TOKEN Failed")
      (CallFunction|FSetWarningChat "TOKEN Failed")
      (bind _returnvalue (Game|GetCurrentLevelName true))
      (if (Utilities|Enum|Equal(Enum) (Variables|VoiceChat|GetEOS%20Room%20Name) _returnvalue)
        (Class|BPIInteractionInterface|BPIFSetVoiceButtonEnabled?(Message) (HUD|GetHUD) true)
        (Variables|VoiceChat|SetConnectedToGlobalChat? false)))))

(event Custom|SendPlayerChatMessage%28Client%29
  (params (TextToSend :type String) (TargetPlayerName :type String))
  ;[1 1 1] Private messaging
  ;;[1 1 1] Process Player Chats
  (Default|SendPlayerChatMessage(Server) (Variables|Default|GetBP_ChatComponent) (Variables|AdvanceChat|GetPlayerName) TextToSend self TargetPlayerName))

(event Custom|Init%20Voice
  (params (Username :type String))
  ;[1 1 1] Init EOS Voice
  (Variables|VoiceChat|SetEOS%20Username Username)
  (bind _returnvalue (Class|EVIKFunctions|InitializeEOSVoiceChat))
  (if _returnvalue
    (Class|EVIKFunctions|ConnectVoiceChat (delegate Custom|ConnectToEOSVoiceChat_Result))
    (else
      (Development|PrintString "Initializing EOS Failed" false true "(R=1.000000,G=0.772624,B=0.000000,A=1.000000)" 5.0)
      (CallFunction|FSetWarningChat "Initializing EOS Failed")
      (Class|BPIInteractionInterface|BPIFSetVoiceButtonEnabled?(Message) (HUD|GetHUD) true)
      (Variables|VoiceChat|SetConnectedToGlobalChat? false))))

(event Custom|ConnectToEOSVoiceChat_Result
  (params (bWasSuccess :type Boolean) (Result :type EEVIKResultCodes%20Enum :default "Success"))
  ;[1 1 1] Init EOS Voice
  (Development|PrintString (Utilities|String|Append "Connect Success: " (Utilities|String|ToString(Boolean) bWasSuccess)))
  (if bWasSuccess
    (Class|EVIKFunctions|LoginEOSVoiceChat (Variables|VoiceChat|GetEOS%20Username) (delegate Custom|LoginToEOSVoiceChat_Result))
    (else
      (Development|PrintString "Connect To EOS VoiceChat Failed" false true "(R=1.000000,G=0.861521,B=0.000000,A=1.000000)" 5.0)
      (CallFunction|FSetWarningChat "Connect To EOS VoiceChat Failed")
      (Class|BPIInteractionInterface|BPIFSetVoiceButtonEnabled?(Message) (HUD|GetHUD) true)
      (Variables|VoiceChat|SetConnectedToGlobalChat? false))))

(event Custom|LoginToEOSVoiceChat_Result
  (params (bWasSuccess :type Boolean) (Result :type EEVIKResultCodes%20Enum :default "Success"))
  ;[1 1 1] Init EOS Voice
  (if bWasSuccess
    (Development|PrintString "Sukses Login" true true "(R=1.000000,G=0.861521,B=0.000000,A=1.000000)" 5.0)
    (CallFunction|FSetWarningChat "Sukses Login")
    (Utilities|FlowControl|Delay 0.5)
    (bind _returnvalue (Game|GetCurrentLevelName true))
    (CallFunction|GetRoomToken (Utilities|String|ToLower _returnvalue))
    (else
      (Development|PrintString "LoginToEOSVoiceChat Failed" true true "(R=1.000000,G=0.861521,B=0.000000,A=1.000000)" 5.0)
      (CallFunction|FSetWarningChat "LoginToEOSVoiceChat Failed")
      (Class|BPIInteractionInterface|BPIFSetVoiceButtonEnabled?(Message) (HUD|GetHUD) true)
      (Variables|VoiceChat|SetConnectedToGlobalChat? false))))

(event Custom|Checking%20Data%20From%20Widget
  (Development|PrintText (Utilities|Text|FormatText "Checking data: 
Destination Server:  {dest} 
AWS Server: {AWS} 
PC Server Tag: {tag}" (Variables|Default|Gettri_DestinationServer) (Variables|Default|Gettri_aws_Server) (Variables|Default|GetPC%20ServerTag)) false true "(R=1.000000,G=0.000000,B=0.816841,A=1.000000)" 1e+01))

(event Custom|SetPlayerName
  (params (NewName :type String))
  ;[1 1 1] Set player name
  (CallFunction|OCSetPlayerName))

(event Custom|SR_Ngasi_GI
  (params (ServerTag :type Name))
  (Development|PrintString (Utilities|String|Append "SR_Ngasi_GI: " (Utilities|String|ToString(Name) ServerTag)) false)
  (bind _asbp_gm_tri (Utilities|Casting|CastToBP_GM_Tri (Game|GetGameMode)))
  (Default|NerimaGI _asbp_gm_tri ServerTag))

(event Custom|UpdateTeamID
  ;[1 0 0] This code has been added to test messaging among team members in the messaging system.
  (Variables|AdvanceChat|SetTeamID "2"))

(event EventBPIFCheckPS
  (bind _returnvalue (UserInterface|CreateWidget "/Game/Blueprints/Widgets/Voice/WBP_VoiceNotif.WBP_VoiceNotif_C" 0 "wewew"))
  (UserInterface|Viewport|AddtoViewport _returnvalue 0))

(event EventBeginPlay
  (bind _hud (Variables|AdvanceChat|GetHud))
  (bind _wbp_chatplayersbox (Variables|/Game/AdvancedChatSystem/Blueprint/UI/WBP_HUD.WBP_HUD_C|GetWBP_ChatPlayersBox _hud))
  (bind _asbp_game_instance (Utilities|Casting|CastToBP_GameInstance (Game|GetGameInstance)))
  (Variables|Default|SetAs%20BP%20Game%20Instance _asbp_game_instance)
  (if (not (Math|Boolean|ANDBoolean (Class|VRExpansionFunctionLibrary|GetIsHMDConnected) (not (Class|KismetSystemLibrary|IsUnattended)) (Class|VRExpansionFunctionLibrary|IsinVREditorPrevieworGame))) ; If is in VR
    (Utilities|DetectDeviceType
      (:Out%20Put
        (Variables|Default|SetbShowMouseCursor true)
        ;[0 0.1433 1] Advance Chat
        (CallFunction|InitializeHUD)
        (Default|EventCallGlobalChat _wbp_chatplayersbox)
        (Widget|SetVisibility _hud "SelfHitTestInvisible")
        (Widget|SetVisibility _wbp_chatplayersbox "Collapsed")
        (Utilities|FlowControl|Delay 5.0)
        (Development|ExecuteConsoleCommand "r.Streaming.PoolSize 1000" 0)
        (CallFunction|FScalability)
        ;[1 1 1] Disconnect Voice when enter new Map
        (bind _returnvalue (Class|EVIKFunctions|GetAllRooms))
        (for _array_element _returnvalue
          ;;[1 1 1] Leave All Connected Rooms
          (Class|EVIKFunctions|LeaveEOSRoom _array_element (delegate Custom|EOS%20Leave%20EOS%20Voice%20Room)))
        (Utilities|FlowControl|Sequence
          (:then_0
            (Development|PrintString "All Voice room has been disconnected" true true "(R=0.000000,G=0.038916,B=1.000000,A=1.000000)" 5.0))
          (:then_1
            (CallFunction|FScalability)))))))

(event EventTick
  (params (DeltaSeconds :type Float%20%28single-precision%29)))

(event EventBPIFSetScalability
  (params (Scalability :type Integer))
  (CallFunction|FScalability))

(event EventBPIFToggleGlobaChatVisibility
  (params (Visible? :type Boolean))
  (bind _hud (Variables|AdvanceChat|GetHud))
  (if Visible?
    (Widget|SetVisibility _hud "SelfHitTestInvisible")
    (Widget|SetVisibility (Variables|/Game/AdvancedChatSystem/Blueprint/UI/WBP_HUD.WBP_HUD_C|GetWBP_ChatPlayersBox _hud) "Collapsed")
    (else
      (Widget|SetVisibility _hud "Collapsed")
      (Widget|SetVisibility (Variables|/Game/AdvancedChatSystem/Blueprint/UI/WBP_HUD.WBP_HUD_C|GetGlobalChatWbp _hud) "SelfHitTestInvisible"))))

(event Input|KeyboardEvents|DebugKeyK
  (params (Key :type Key%20Structure :default "None") (ActionValue :type Input%20Action%20Value%20Structure))
  ;[1 0 0] Player name controll
)

(event Input|KeyboardEvents|DebugKeyK
  (params (Key :type Key%20Structure :default "None") (ActionValue :type Input%20Action%20Value%20Structure))
  ;[1 1 1] PlayerNameDebug
  (:Pressed
    (Development|PrintString (Variables|AdvanceChat|GetPlayerName))))

(event Input|KeyboardEvents|AnyKey
  (params (Key :type Key%20Structure :default "None"))
  (bind _as_bp_game_instance (Variables|Default|GetAs%20BP%20Game%20Instance))
  (:Pressed
    (if (Utilities|String|Contains (Utilities|String|ToString(Text) (Class|KismetInputLibrary|KeyGetDisplayName Key true)) "Gamepad")
      (Variables|/Game/Blueprints/Subsystem/BP_GameInstance.BP_GameInstance_C|SetUseGamepad _as_bp_game_instance true)
      (else
        (Variables|/Game/Blueprints/Subsystem/BP_GameInstance.BP_GameInstance_C|SetUseGamepad _as_bp_game_instance false)))))

(event Input|KeyboardEvents|NumPadZero
  (params (Key :type Key%20Structure :default "None"))
  (:Pressed
    (bind _returnvalue (Game|GetCurrentLevelName true))
    ;[1 1 1] Set Scalability by pressing Android Back Button
    (if (not (Utilities|Enum|Equal(Enum) _returnvalue "MainWorld"))
      (Variables|Default|GetWBP_QuitGame
        (:then
          (if (Widget|IsVisible (Variables|Default|GetWBP_QuitGame))
            (Widget|SetVisibility (Variables|Default|GetWBP_QuitGame) "Collapsed")
            (Audio|PlaySound2D "/Engine/VREditor/Sounds/UI/Click_on_Button.Click_on_Button" 1.0 1.0 0.0 0 0)
            (else
              (Widget|SetVisibility (Variables|Default|GetWBP_QuitGame) "SelfHitTestInvisible")
              (Audio|PlaySound2D "/Engine/VREditor/Sounds/UI/Camera_Shutter.Camera_Shutter" 1.0 1.0 0.0 0 0 :!label _label))))
        (:else
          (bind _returnvalue_2 (UserInterface|CreateWidget "/Game/Blueprints/Widgets/WBP_QuitGameNotif.WBP_QuitGameNotif_C"))
          (bind _output_get (Variables|Default|SetWBP_QuitGame _returnvalue_2))
          (UserInterface|Viewport|AddtoViewport _output_get 0)
          (goto _label))))))

(event Input|KeyboardEvents|1
  (params (Key :type Key%20Structure :default "None"))
  (:Pressed
    (bind _asbp_player_character (Utilities|Casting|CastToBP_PlayerCharacter (Game|GetPlayerCharacter 0)))
    (Default|SREquipWeapon _asbp_player_character)))

(event Input|KeyboardEvents|3
  (params (Key :type Key%20Structure :default "None"))
  (:Pressed
    (CallFunction|GetGM)))

(event Input|KeyboardEvents|2
  (params (Key :type Key%20Structure :default "None"))
  (:Pressed
    (bind _returnvalue (Game|GetCurrentLevelName true))
    (Development|PrintString _returnvalue)))

(event Input|KeyboardEvents|4
  (params (Key :type Key%20Structure :default "None"))
  (:Pressed
    (Development|PrintString (Utilities|String|ToString(Vector) (Transformation|GetActorLocation (Pawn|GetControlledPawn self))) true true "(R=0.000000,G=0.024146,B=1.000000,A=1.000000)" 1e+01)))

(event Input|KeyboardEvents|7
  (params (Key :type Key%20Structure :default "None"))
  (:Pressed
    (CallFunction|ControlVoiceVolume)))

(event Input|KeyboardEvents|AndroidBack
  (params (Key :type Key%20Structure :default "None"))
  (:Pressed
    (bind _returnvalue (Game|GetCurrentLevelName true))
    ;[1 1 1] Set Scalability by pressing Android Back Button
    (if (not (Utilities|Enum|Equal(Enum) _returnvalue "MainWorld"))
      (Variables|Default|GetWBP_QuitGame
        (:then
          (if (Widget|IsVisible (Variables|Default|GetWBP_QuitGame))
            (Widget|SetVisibility (Variables|Default|GetWBP_QuitGame) "Collapsed")
            (Audio|PlaySound2D "/Engine/VREditor/Sounds/UI/Click_on_Button.Click_on_Button" 1.0 1.0 0.0 0 0)
            (else
              (Widget|SetVisibility (Variables|Default|GetWBP_QuitGame) "SelfHitTestInvisible")
              (Audio|PlaySound2D "/Engine/VREditor/Sounds/UI/Camera_Shutter.Camera_Shutter" 1.0 1.0 0.0 0 0 :!label _label))))
        (:else
          (bind _returnvalue_2 (UserInterface|CreateWidget "/Game/Blueprints/Widgets/WBP_QuitGameNotif.WBP_QuitGameNotif_C"))
          (bind _output_get (Variables|Default|SetWBP_QuitGame _returnvalue_2))
          (UserInterface|Viewport|AddtoViewport _output_get 0)
          (goto _label))))))

(fn ConstructionScript)

(fn FSetWarningChat
  (params (TextWarningChat :type Text))
  (Class|BPIInteractionInterface|BPIFFSetTextWarningChat(Message) (HUD|GetHUD) TextWarningChat))

(fn CallIUpListOfPlayersinGame
  (params (WBP_ChatPlayersBox :type WBP%20Chat%20Players%20Box%20Object%20Reference))
  (bind _asbp_gameplay_game_mode (Utilities|Casting|CastToBP_GameplayGameMode (Game|GetGameMode)))
  (for _array_element (Variables|/Game/Blueprints/GameMode/BP_GameplayGameMode.BP_GameplayGameMode_C|GetConnectedPlayers _asbp_gameplay_game_mode)
    (if (!= _array_element self)
      (CallFunction|SetEntryPlayers (Variables|BP_PlayerController_C|GetPlayerName _array_element) _array_element))))

(fn FScalability
  (if (== (Variables|Default|GetScalability) 2)
    (Variables|Default|SetScalability 3)
    (else
      (Variables|Default|SetScalability 2)))
  (Development|ExecuteConsoleCommand (Utilities|String|Append "scalability " (Utilities|String|ToString(Integer) (Variables|Default|GetScalability))) self)
  (Development|PrintString "scalability set" false))

(fn DetectDeviceTypefromCharacter
  (Utilities|DetectDeviceType))

(fn BPIFGetInventoryArray
  (return 0 0 0))

(fn BPIFGetPoints
  (return 0 0))