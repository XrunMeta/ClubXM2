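; Game mode that runs a maintenance check against a web API at startup and registers players as they log in.
; BeginPlay sends a VaRest GET getMaintenance request, and its completion event only prints client validity from the returned status.
; PostLogin adds each player's BP_PlayerState and info struct to the PlayerInfoSubsystem's AllPlayersMap.
; An unconnected OpenWeatherMap test call and its callback remain in the graph.
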(event `RestCallback`
  (params (Request :type "VaRestRequestJSON Object Reference"))
  ;[1 1 1] Test, and it works!
  (bind _returnvalue (`VaRestJsonValue.AsObject` (`|GetArrayItem` (`VaRestJsonObject.GetArrayField` (`VaRestRequestJSON.GetResponseObject` Request) "weather"))))
  (`KismetSystemLibrary.PrintString` (`VaRestJsonObject.GetStringField` _returnvalue "description")))

(event `self.ReceiveBeginPlay`
  (bind _returnvalue (`VaRestSubsystem.ConstructVaRestRequestExt` (subsystem `VaRestSubsystem`) "GET" "x_www_form_urlencoded_url"))
  (`VaRestRequestJSON.ProcessURL` _returnvalue (`KismetTextLibrary.Conv_TextToString` (`|FormatText` "{URL}?action=getMaintenance" (`self.URL API`))))
  (add `VaRestRequestJSON.OnRequestComplete` _returnvalue (delegate `OnRequestComplete_Event`)))

(event `OnRequestComplete_Event`
  (params (Request :type "VaRestRequestJSON Object Reference"))
  (bind _returnvalue (`VaRestJsonValue.AsObject` (`|GetArrayItem` (`VaRestJsonObject.GetArrayField` (`VaRestRequestJSON.GetResponseObject` Request) "data"))))
  (if (`KismetStringLibrary.EqualEqual_StrStr` (`VaRestJsonObject.GetStringField` _returnvalue "status") "1")
    (`KismetSystemLibrary.PrintString` "Client's invalid" true true (struct :`R` 1.0 :`B` 0.037924 :`A` 1.0))
    (else
      (`KismetSystemLibrary.PrintString` "Client's Valid" true true (struct :`R` 0.06965 :`G` 1.0 :`A` 1.0)))))

(event `self.K2_PostLogin`
  (params (NewPlayer :type "PlayerController Object Reference"))
  (bind _returnvalue (pcsubsystem `PlayerInfoSubsystem` NewPlayer))
  (bind _allplayersmap (`PlayerInfoSubsystem.AllPlayersMap` _returnvalue))
  (if (`KismetSystemLibrary.IsValid` _returnvalue)
    (bind _asbp_player_state (cast `/Game/Blueprints/PlayerState/BP_PlayerState` (`Controller.PlayerState` NewPlayer)))
    (`BlueprintMapLibrary.Map_Add` _allplayersmap _asbp_player_state (`PlayerInfoSubsystem.PlayerInfoStruct` _returnvalue))
    (`BlueprintMapLibrary.Map_Values` _allplayersmap)
    (`KismetSystemLibrary.PrintString` (`KismetSystemLibrary.GetDisplayName` _asbp_player_state))
    (else
      (`KismetSystemLibrary.PrintString` "Subsystem's Nullptr" true true (struct :`R` 1.0 :`B` 0.014578 :`A` 1.0)))))

(fn `UserConstructionScript`)