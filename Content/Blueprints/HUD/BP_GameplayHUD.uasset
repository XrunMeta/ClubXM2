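; Gameplay HUD that, outside VR, creates the main widget and a collapsed voice-chat debug widget in landscape orientation.
; Events and interface calls relay player lists, login logs, friend requests, chat state, interact prompts, scene captures and settings owner to child widgets.
; Bound dispatchers hide the gameplay UI or fill its server IP and tag texts; character-select apply and cancel both restore the gameplay canvas.
; Inventory and points getters are stubs.
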(event `self.ReceiveBeginPlay`
  ;[0 0 0] Initialize
  (if (not (and (`VRExpansionFunctionLibrary.GetIsHMDConnected`) (not (`KismetSystemLibrary.IsUnattended`)) (`VRExpansionFunctionLibrary.IsInVREditorPreviewOrGame`)))
    ;;[1 1 1] Main Widget
    (`BlueprintPlatformLibrary.SetAllowedDeviceOrientation` "LandscapeSensor")
    (bind _returnvalue (`|CreateWidget` "/Game/Blueprints/Widgets/WBP_MainWidget.WBP_MainWidget_C" (`self.GetOwningPlayerController`)))
    (bind _output_get (set `self.BP_MainWidget` _returnvalue))
    (`UserWidget.AddToViewport` _output_get 0)
    ;;[1 0.04956 0] Tri Debug for Voice Chat (DEVELOPMENT ONLY. Later can be deleted)
    (bind _returnvalue_2 (`|CreateWidget` "/Game/Blueprints/Widgets/WBP_TriDebug.WBP_TriDebug_C" (`self.PlayerOwner`)))
    (`UserWidget.AddToViewport` _returnvalue_2 0)
    (set `self.As WBP Tri Debug` _returnvalue_2)
    (`Widget.SetVisibility` _returnvalue_2 "Collapsed")
    (add `self.OnHideIPAdress` (delegate `OnHideIPAdress_Event`))
    (add `self.OnSendIPAdress` (delegate `OnSendIPAdress_Event`))))

(event `OnHideIPAdress_Event`
  ;[0 0 0] Initialize
  (bind _bp_mainwidget (`self.BP_MainWidget`)
    (:`then`
      (bind _wbp_gameplayui (`/Game/Blueprints/Widgets/WBP_MainWidget.WBP_GameplayUI` _bp_mainwidget)
        (:`then`
          (`Widget.SetVisibility` _wbp_gameplayui "Hidden"))
        (:`else`)))
    (:`else`)))

(event `OnSendIPAdress_Event` :!signature `self.OnSendIPAdress`
  (params (DestinationIPAdress :type String) (AWSIPAdress :type String) (ServerTag :type Name))
  ;[0 0 0] Initialize
  (`self.SendIPAdress` DestinationIPAdress AWSIPAdress ServerTag))

(event `UpdateListPlayers`
  (params (PlayerDataArray :type "Array of /Game/Blueprints/Structure/S_PlayerData Structure"))
  ;[0 0 0] Update List Player
  (bind _bp_mainwidget (`self.BP_MainWidget`)
    (:`then`
      (bind _wbp_mainmenu (`/Game/Blueprints/Widgets/WBP_MainWidget.WBP_MainMenu` _bp_mainwidget)
        (:`then`
          (bind _wbp_playerslist (`/Game/Blueprints/Widgets/WBP_MainMenu.WBP_PlayersList` _wbp_mainmenu)
            (:`then`
              (`/Game/Blueprints/Widgets/WBP_PlayersList.UpdateListPlayerOption` _wbp_playerslist PlayerDataArray)
              (`self.UpdateLogActivity` PlayerDataArray true))
            (:`else`)))
        (:`else`)))
    (:`else`)))

(event `UpdateLogActivity`
  (params (PlayerData :type "Array of /Game/Blueprints/Structure/S_PlayerData Structure") (IsLogin :type Boolean))
  ;[0 0 0] Update Log Activity
  (bind _bp_mainwidget (`self.BP_MainWidget`)
    (:`then`
      (bind _wbp_log (`/Game/Blueprints/Widgets/WBP_MainWidget.WBP_Log` _bp_mainwidget)
        (:`then`
          (`/Game/Blueprints/Widgets/WBP_Log.UpdateLogActivity` _wbp_log PlayerData IsLogin))
        (:`else`)))
    (:`else`)))

(event `ActivateNotificationRequest`
  (params (ReceiverPlayer :type "/Game/Blueprints/Structure/S_PlayerData Structure"))
  (bind _bp_mainwidget (`self.BP_MainWidget`)
    (:`then`
      (bind _wbp_mainmenu (`/Game/Blueprints/Widgets/WBP_MainWidget.WBP_MainMenu` _bp_mainwidget)
        (:`then`
          (bind _wbp_playerslist (`/Game/Blueprints/Widgets/WBP_MainMenu.WBP_PlayersList` _wbp_mainmenu)
            (:`then`
              (`/Game/Blueprints/Widgets/WBP_PlayersList.UpdateRequestFriends` _wbp_playerslist ReceiverPlayer))
            (:`else`)))
        (:`else`)))
    (:`else`)))

(event `SetInteractableVisibility`
  (params (Visibile :type Boolean))
  ;[0 0 0] Setup Visibility Popup Widget
  (bind _bp_mainwidget (`self.BP_MainWidget`)
    (:`then`
      (bind _wbp_mainmenu (`/Game/Blueprints/Widgets/WBP_MainWidget.WBP_MainMenu` _bp_mainwidget)
        (:`then`
          (if Visibile
            (bind _borderinteract (`/Game/Blueprints/Widgets/WBP_MainMenu.BorderInteract` _wbp_mainmenu))
            (`Widget.SetVisibility` _borderinteract "Visible")
            (else
              (`Widget.SetVisibility` _borderinteract "Collapsed"))))
        (:`else`)))
    (:`else`)))

(event `SetSceneCaptureOwner`
  (params (SceneCaptureComp :type "SceneCaptureComponent2D Object Reference") (OwnerCharacter :type "/Game/Blueprints/Character/BP_PlayerCharacter Object Reference"))
  ;[0 0 0] Setup SceneCapture2D Cam
  (bind _bp_mainwidget (`self.BP_MainWidget`)
    (:`then`
      (bind _wbp_characterselect (`/Game/Blueprints/Widgets/WBP_MainWidget.WBP_CharacterSelect` _bp_mainwidget)
        (:`then`
          (`/Game/Blueprints/Widgets/WBP_CharacterSelect.SetRenderTarget2D` _wbp_characterselect SceneCaptureComp OwnerCharacter))
        (:`else`)))
    (:`else`)))

(event `SetOwnerOfSettings`
  (params (OwnerCharacter :type "/Game/Blueprints/PlayerState/BP_PlayerState Object Reference"))
  ;[0 0 0] Setup Owner Character on Settings
  (bind _bp_mainwidget (`self.BP_MainWidget`)
    (:`then`
      (bind _wbp_settings (`/Game/Blueprints/Widgets/WBP_MainWidget.WBP_Settings` _bp_mainwidget)
        (:`then`
          (`/Game/Blueprints/Widgets/WBP_Settings.GetOwner` _wbp_settings OwnerCharacter))
        (:`else`)))
    (:`else`)))

(event `/Game/Blueprints/Interface/BPI_InteractionInterface.BPIF_FSetTextWarningChat`
  (params (WarningText :type Text))
  (`/Game/Blueprints/Widgets/WBP_MainMenu.FSet_ChatWarningtext` (`/Game/Blueprints/Widgets/WBP_MainWidget.WBP_MainMenu` (`self.BP_MainWidget`)) WarningText))

(event `/Game/Blueprints/Interface/BPI_InteractionInterface.BPIF_SetVoiceButtonEnabled?`
  (params (`Enabled?` :type Boolean))
  (`Widget.SetIsEnabled` (`/Game/Blueprints/Widgets/WBP_MainMenu.ButtonVoiceOrText` (`/Game/Blueprints/Widgets/WBP_MainWidget.WBP_MainMenu` (`self.BP_MainWidget`))) `Enabled?`))

(event `/Game/Blueprints/Interface/BPI_CharacterSelect.BPIF_CancelCharacterSelect`
  (params (`Current Mesh` :type "SkeletalMesh Object Reference"))
  ;[1 1 1] Make visible Main Menu and Action Menu and Hide Character Select Widget
  ; Triggered from WBP_CharacterSelect
  (if (not (and (`VRExpansionFunctionLibrary.GetIsHMDConnected`) (not (`KismetSystemLibrary.IsUnattended`)) (`VRExpansionFunctionLibrary.IsInVREditorPreviewOrGame`))) :!label _label
    (`Widget.SetVisibility` (`/Game/Blueprints/Widgets/WBP_MainWidget.CanvasGameplay` (`self.BP_MainWidget`)) "SelfHitTestInvisible")
    (`Widget.SetVisibility` (`/Game/Blueprints/Widgets/WBP_MainWidget.WBP_CharacterSelect` (`self.BP_MainWidget`)) "Collapsed")))

(event `/Game/Blueprints/Interface/BPI_CharacterSelect.BPIF_ApplyCharacterSelect`
  (params (Selected_Skeletalmesh :type "SkeletalMesh Object Reference"))
  ;[1 1 1] Make visible Main Menu and Action Menu and Hide Character Select Widget
  ; Triggered from WBP_CharacterSelect
  (goto _label))

(fn `BPIF_GetInventoryArray`
  (returns (Inventory_Roses :type "Array of Integer") (Inventory_Guns :type "Array of Integer") (Inventory_AvatarItems :type "Array of Integer"))
  (return))

(fn `BPIF_GetPoints`
  (returns (mXRUN :type Integer) (XRUN :type Integer))
  (return 0 0))

(fn `SendIPAdress`
  (params (DestinationIPAdress :type String) (AWSIPAdress :type String) (ServerTag :type Name))
  (bind _bp_mainwidget (`self.BP_MainWidget`)
    (:`then`
      (bind _wbp_gameplayui (`/Game/Blueprints/Widgets/WBP_MainWidget.WBP_GameplayUI` _bp_mainwidget)
        (:`then`
          (`TextBlock.SetText` (`/Game/Developers/metadevwin003/WBP_GameplayUI.Text_DestinationServer` _wbp_gameplayui) (`KismetTextLibrary.Conv_StringToText` DestinationIPAdress))
          (`TextBlock.SetText` (`/Game/Developers/metadevwin003/WBP_GameplayUI.Text_DestinationServerBtn` _wbp_gameplayui) (`KismetTextLibrary.Conv_StringToText` DestinationIPAdress))
          (`TextBlock.SetText` (`/Game/Developers/metadevwin003/WBP_GameplayUI.Text_AWSServerBtn` _wbp_gameplayui) (`KismetTextLibrary.Conv_StringToText` AWSIPAdress))
          (`TextBlock.SetText` (`/Game/Developers/metadevwin003/WBP_GameplayUI.Text_ServerTag` _wbp_gameplayui) (`KismetTextLibrary.Conv_StringToText` (`KismetStringLibrary.Conv_NameToString` ServerTag))))
        (:`else`)))
    (:`else`)))

(fn `UserConstructionScript`)