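; Hinged door for a multiplayer game that opens and closes on OpenDoorR, consuming the player's key to unlock it if locked.
; Front and Back overlaps record the player's side, choosing which timeline swings the mesh from closed.
; A one-sided door refuses opening from the back until a front opening clears that flag.
; Current yaw decides between opening and reversing the matching timeline at ±90 degrees to close.
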(event `OpenDoorR`
  (params (Character_Ref :type "/Game/TPS_Multiplayer_Pack/Blueprints/PlayersCharacter/PB_PlayerCharacter Object Reference"))
  (bind _door (`self.Door`))
  (bind _player_ref (`self.Player_Ref`))
  (bind _yaw (.yaw (`SceneComponent.RelativeRotation` (`self.Door`))))
  (set `self.Player_Ref` Character_Ref)
  (if (`self.IsLocked?`)
    (if (`/Game/TPS_Multiplayer_Pack/Blueprints/PlayersCharacter/PB_PlayerCharacter.PlayerHasKey?` _player_ref)
      (set `/Game/TPS_Multiplayer_Pack/Blueprints/PlayersCharacter/PB_PlayerCharacter.PlayerHasKey?` false _player_ref)
      (set `self.IsLocked?` false)
      (if (`KismetMathLibrary.NearlyEqual_FloatFloat` _yaw 0.0 0.1) :!label _label
        (if (`self.FrontDoor?`)
          (bind (_direction _newtrack_1) (`Timeline|Timeline_0` :!via `PlayFromStart` :!label _label_2)
            (:`Update`
              (`SceneComponent.K2_SetRelativeRotation` _door (`KismetMathLibrary.MakeRotator` 0.0 0.0 _newtrack_1) false false)
              (set `self.OneSidedDoor?` false)))
          (elif (not (`self.OneSidedDoor?`))
            (bind (_direction_2 _newtrack_3) (`Timeline|Timeline_1` :!label _label_3)
              (:`Update`
                (`SceneComponent.K2_SetRelativeRotation` _door (`KismetMathLibrary.MakeRotator` 0.0 0.0 _newtrack_3) false false)))))
        (elif (`KismetMathLibrary.NearlyEqual_FloatFloat` _yaw 90.0 0.1)
          (goto _label_2 :!via `Reverse`)
          (elif (`KismetMathLibrary.NearlyEqual_FloatFloat` _yaw -90.0 0.1)
            (goto _label_3 :!via `Reverse`)))))
    (else
      (goto _label))))

(event `self.Back.OnComponentBeginOverlap`
  (params (OverlappedComponent :type "PrimitiveComponent Object Reference") (OtherActor :type "Actor Object Reference") (OtherComp :type "PrimitiveComponent Object Reference") (OtherBodyIndex :type Integer) (bFromSweep :type Boolean) (SweepResult :type "HitResult Structure (by ref)"))
  (cast `/Game/TPS_Multiplayer_Pack/Blueprints/PlayersCharacter/PB_PlayerCharacter` OtherActor)
  (set `self.FrontDoor?` false))

(event `self.Front.OnComponentBeginOverlap`
  (params (OverlappedComponent :type "PrimitiveComponent Object Reference") (OtherActor :type "Actor Object Reference") (OtherComp :type "PrimitiveComponent Object Reference") (OtherBodyIndex :type Integer) (bFromSweep :type Boolean) (SweepResult :type "HitResult Structure (by ref)"))
  (cast `/Game/TPS_Multiplayer_Pack/Blueprints/PlayersCharacter/PB_PlayerCharacter` OtherActor)
  (set `self.FrontDoor?` true))

(fn `UserConstructionScript`)