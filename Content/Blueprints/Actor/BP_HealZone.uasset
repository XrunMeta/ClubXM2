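; BP_HealZone is a zone actor that gradually heals the player character while they stand inside its sphere.
; Sphere overlap events store or clear the BP_PlayerCharacter reference and toggle a healing flag.
; A self-calling Healing event applies SRHeal on a delayed loop until health reaches the cap or the player leaves, printing debug messages along the way.
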(event `self.Sphere1.OnComponentBeginOverlap`
  (params (OverlappedComponent :type "PrimitiveComponent Object Reference") (OtherActor :type "Actor Object Reference") (OtherComp :type "PrimitiveComponent Object Reference") (OtherBodyIndex :type Integer) (bFromSweep :type Boolean) (SweepResult :type "HitResult Structure (by ref)"))
  (bind _asbp_player_character (cast `/Game/Blueprints/Character/BP_PlayerCharacter` OtherActor))
  (set `self.As BP Player Character` _asbp_player_character)
  (set `self.Helaing?` true)
  (`self.Healing`))

(event `self.Sphere1.OnComponentEndOverlap`
  (params (OverlappedComponent :type "PrimitiveComponent Object Reference") (OtherActor :type "Actor Object Reference") (OtherComp :type "PrimitiveComponent Object Reference") (OtherBodyIndex :type Integer))
  (cast `/Game/Blueprints/Character/BP_PlayerCharacter` OtherActor)
  (set `self.As BP Player Character` null)
  (set `self.Helaing?` false))

(event `Healing`
  (bind _as_bp_player_character (`self.As BP Player Character`))
  (bind _health (`/Game/Blueprints/Character/BP_PlayerCharacter.Health` _as_bp_player_character))
  (if (`self.Helaing?`)
    (`KismetSystemLibrary.PrintString` "Heal Process")
    (if (< _health 100.0)
      (`/Game/Blueprints/Character/BP_PlayerCharacter.SR_Heal` _as_bp_player_character 10.0)
      (`KismetSystemLibrary.PrintString` (`KismetStringLibrary.Conv_DoubleToString` _health))
      (`KismetSystemLibrary.Delay` 2.0)
      (`self.Healing`)
      (else
        (`KismetSystemLibrary.PrintString` "Maximum")))
    (else
      (`KismetSystemLibrary.PrintString` "Heal ended"))))

(fn `UserConstructionScript`)