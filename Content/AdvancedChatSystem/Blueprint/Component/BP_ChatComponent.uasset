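; Chat component that routes player messages on the server as global, team, nearby or private chat.
; Server events switch on message type: global reaches the game mode's connected players, team matches controllers by TeamID, and nearby distance-checks BP_Man_1 actors against the sender's pawn.
; Private messages update the sender and any controller with the target name.
; Delivery calls chat log updates on BP_PlayerController; an empty TeamID updates only the sender.
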(event `SendPlayerChatMessage(Server)`
  (params (PlayerName :type String) (TextToSend :type String) (Controller :type "Controller Object Reference") (TargetPlayerName :type String))
  ;[0.1615 0.006727 0.006727] Set player messeage
  (`self.SendPlayerChatMessage` PlayerName TextToSend Controller TargetPlayerName))

(event `SendGlobalChatMessage(Server)`
  (params (PlayerName :type String) (TextToSend :type String) (Controller :type "Controller Object Reference") (`Message Type` :type "/Game/AdvancedChatSystem/Blueprint/Enum/E_MessageType Enum" :default "NewEnumerator0") (TeamID :type String))
  ;[1 1 1] Type Check
  (switch `/Game/AdvancedChatSystem/Blueprint/Enum/E_MessageType` `Message Type`
    (:`NewEnumerator0`
      (`self.SendToGlobalMessage` PlayerName TextToSend))
    (:`NewEnumerator1`
      (`self.SendToTeamMessage` PlayerName TextToSend TeamID Controller))
    (:`NewEnumerator2`
      (`self.SendToNearbyDistanceMessage` PlayerName TextToSend Controller))))

(event `SendToGlobalMessage`
  (params (PlayerName :type String) (TextToSend :type String))
  ;[1 1 1] Process Global Chats
  (bind _asbp_gameplay_game_mode (cast `/Game/Blueprints/GameMode/BP_GameplayGameMode` (`GameplayStatics.GetGameMode`)))
  (for _array_element (`/Game/Blueprints/GameMode/BP_GameplayGameMode.ConnectedPlayers` _asbp_gameplay_game_mode)
    (`/Game/Blueprints/PlayerController/BP_PlayerController.UpdateChatLog` _array_element PlayerName TextToSend "NewEnumerator0")))

(event `SendToNearbyDistanceMessage`
  (params (PlayerName :type String) (TextToSend :type String) (Controller :type "Controller Object Reference"))
  (bind _returnvalue (`Controller.K2_GetPawn` Controller))
  ;[1 1 1] Nearby Distance
  (`/Engine/EditorBlueprintResources/StandardMacros.IsValid` _returnvalue ; nearby
    (:`Is Valid`
      (bind _outactors (`GameplayStatics.GetAllActorsOfClass` "/Game/Blueprints/Character/BP_Man_1.BP_Man_1_C"))
      (for _array_element _outactors
        (if (< (`KismetMathLibrary.Vector_Distance` (`Actor.K2_GetActorLocation` _array_element) (`Actor.K2_GetActorLocation` _returnvalue)) (`self.NearbyDistance`))
          (bind _asbp_player_controller (cast `/Game/Blueprints/PlayerController/BP_PlayerController` (`Pawn.GetController` _array_element)))
          (`/Game/Blueprints/PlayerController/BP_PlayerController.UpdateChatLog` _asbp_player_controller PlayerName TextToSend "NewEnumerator2"))))))

(event `SendToTeamMessage`
  (params (PlayerName :type String) (TextToSend :type String) (TeamID :type String) (Target :type "Controller Object Reference"))
  ;[1 1 1] Team Chat
  (if (!= TeamID "")
    (bind _outactors (`GameplayStatics.GetAllActorsOfClass` "/Game/Blueprints/PlayerController/BP_PlayerController.BP_PlayerController_C"))
    (for _array_element _outactors
      (if (`KismetStringLibrary.EqualEqual_StrStr` (`/Game/Blueprints/PlayerController/BP_PlayerController.TeamID` _array_element) TeamID)
        (`/Game/Blueprints/PlayerController/BP_PlayerController.UpdateChatLog` _array_element PlayerName TextToSend "NewEnumerator1")))
    (else
      (bind _asbp_player_controller (cast `/Game/Blueprints/PlayerController/BP_PlayerController` Target))
      (`/Game/Blueprints/PlayerController/BP_PlayerController.UpdateChatLog` _asbp_player_controller TeamID PlayerName "NewEnumerator1"))))

(fn `SendPlayerChatMessage`
  (params (PlayerName :type String) (Message :type String) (Controller :type "Controller Object Reference") (TargetPlayerName :type String))
  (`|ExecutionSequence`
    (:`then_0`
      (bind _asbp_player_controller (cast `/Game/Blueprints/PlayerController/BP_PlayerController` (`local.Controller`)))
      (`/Game/Blueprints/PlayerController/BP_PlayerController.UpdatePlayerChatLog` _asbp_player_controller (`local.PlayerName`) (`local.Message`) "NewEnumerator0" (`local.TargetPlayerName`)))
    (:`then_1`
      (bind _outactors (`GameplayStatics.GetAllActorsOfClass` "/Game/Blueprints/PlayerController/BP_PlayerController.BP_PlayerController_C"))
      (for _array_element _outactors
        (if (`KismetStringLibrary.EqualEqual_StrStr` (`/Game/Blueprints/PlayerController/BP_PlayerController.PlayerName` _array_element) (`local.TargetPlayerName`))
          (`/Game/Blueprints/PlayerController/BP_PlayerController.UpdatePlayerChatLog` _array_element (`local.PlayerName`) (`local.Message`) "NewEnumerator0" ""))))))