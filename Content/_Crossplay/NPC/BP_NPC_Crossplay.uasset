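; Crossplay NPC Blueprint that picks its skeletal mesh from DT_NPC, using MeshID as an index into the row names.
; BeginPlay assigns the Windows or mobile mesh according to the platform name cached from GI_Multix.
; The construction script labels the NPC with MeshID and previews the mobile mesh on both platform branches.
; Outside Shipping, it sets IsDancing and checks for android.txt in place of the platform name.
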(event `self.ReceiveBeginPlay`
  (bind _outrownames (`DataTableFunctionLibrary.GetDataTableRowNames` "/Game/_Crossplay/DT_NPC.DT_NPC"))
  (bind _returnvalue (`|GetDataTableRow` "/Game/_Crossplay/DT_NPC.DT_NPC" (`|GetArrayItem` _outrownames (`self.MeshID`)))
    (:`then`
      (bind _gi_platform (`self.FCheckGIPlatform`))
      (switch `string` _gi_platform
        (:`Windows`
          (bind (_npc_id _npc_desc _npc_windows _npc_mobile) (break `/Game/_Crossplay/S_NPC` _returnvalue))
          (set `SkeletalMeshComponent.SkeletalMeshAsset` _npc_windows (`self.Mesh`)))
        (:`Android`
          (set `SkeletalMeshComponent.SkeletalMeshAsset` _npc_mobile (`self.Mesh`)))))))

(fn `FCheckGIPlatform`
  (returns (GI_Platform :type String))
  (`self.As GI Multix`
    (:`then`
      (return (`/MultixOnline/Blueprints/GI_Multix.GI_PlatformName` (`self.As GI Multix`))))
    (:`else`
      (bind _asgi_multix (cast `/MultixOnline/Blueprints/GI_Multix` (`GameplayStatics.GetGameInstance`))
        (:`then`
          (set `self.As GI Multix` _asgi_multix)
          (return (`/MultixOnline/Blueprints/GI_Multix.GI_PlatformName` (`self.As GI Multix`))))
        (:`CastFailed`
          (`KismetSystemLibrary.PrintString` (`KismetStringLibrary.Concat_StrStr` (`KismetSystemLibrary.GetDisplayName` self) " Failed to Cast")))))))

(fn `UserConstructionScript`
  (if (not (== (`KismetSystemLibrary.GetBuildConfiguration`) "Shipping"))
    (set `self.IsDancing` true))
  (`TextRenderComponent.K2_SetText` (`self.TextRender`) (`KismetTextLibrary.Conv_IntToText` (`self.MeshID`)))
  (bind _outrownames (`DataTableFunctionLibrary.GetDataTableRowNames` "/Game/_Crossplay/DT_NPC.DT_NPC"))
  (bind _returnvalue (`|GetDataTableRow` "/Game/_Crossplay/DT_NPC.DT_NPC" (`|GetArrayItem` _outrownames (`self.MeshID`)))
    (:`then`
      (if (== (`KismetSystemLibrary.GetBuildConfiguration`) "Shipping")
        (switch `string` (`GameplayStatics.GetPlatformName`)
          (:`Windows`
            (bind (_npc_id _npc_desc _npc_windows _npc_mobile) (break `/Game/_Crossplay/S_NPC` _returnvalue))
            (set `SkeletalMeshComponent.SkeletalMeshAsset` _npc_mobile (`self.Mesh`) :!label _label))
          (:`Android`
            (set `SkeletalMeshComponent.SkeletalMeshAsset` _npc_mobile (`self.Mesh`) :!label _label_2)))
        (elif (`BlueprintPathsLibrary.FileExists` (`KismetStringLibrary.Concat_StrStr` (`KismetSystemLibrary.GetProjectDirectory`) "android.txt"))
          (goto _label_2)
          (else
            (goto _label)))))))