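; Assault weapon paintball projectile that splats paint, deals damage and destroys itself shortly after impact.
; On hit it caches the impact transform, bone and random decal sizes, then ColorChanger picks one of six materials and tints a dynamic instance randomly.
; Enemy characters get decals attached to the hit bone.
; An impact emitter spawns, and DamageInterface actors receive damage range, crit chance, bone, instigator and impulse vector.
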(event `self.Bullet.OnComponentHit`
  (params (HitComponent :type "PrimitiveComponent Object Reference") (OtherActor :type "Actor Object Reference") (OtherComp :type "PrimitiveComponent Object Reference") (NormalImpulse :type "Vector Structure") (Hit :type "HitResult Structure (by ref)"))
  (`self.Location,Rotation,Scale` Hit_ImpactPoint Hit_Normal Hit_HitBoneName)
  (`self.ColorChanger` Hit_HitActor
    (:`Output`
      (`GameplayStatics.SpawnEmitterAtLocation` null (`self.Impact Point`) (`self.Rotation`))
      (if (`KismetSystemLibrary.DoesImplementInterface` Hit_HitActor "/Game/TPS_Multiplayer_Pack/Blueprints/Interfaces/DamageInterface.DamageInterface_C")
        (message `/Game/TPS_Multiplayer_Pack/Blueprints/Interfaces/DamageInterface.TakeDamage` Hit_HitActor (`self.DamageMin`) (`self.DamageMax`) (`self.CritChance`) Hit_HitBoneName (`self.GetInstigator`) (* (`KismetMathLibrary.Normal` (`KismetMathLibrary.GetDirectionUnitVector` Hit_TraceStart Hit_TraceEnd)) (`self.ImpactForce`)))
        (`KismetSystemLibrary.Delay` 0.03)
        (`self.K2_DestroyActor`)
        (else
          (`KismetSystemLibrary.Delay` 0.03)
          (`self.K2_DestroyActor`))))))

(fn `Location,Rotation,Scale`
  (params (Location :type "Vector Structure") (Rotation :type "Vector Structure") (HitBoneName :type Name))
  (set `self.Impact Point` Location)
  (set `self.Rotation` (`KismetMathLibrary.Conv_VectorToRotator` Rotation))
  (set `self.Size` (`KismetMathLibrary.MakeVector` 0.1 (`KismetMathLibrary.RandomFloatInRange` 50.0 100.0) (`KismetMathLibrary.RandomFloatInRange` 50.0 100.0)))
  (set `self.OnPlayerSize` (`KismetMathLibrary.MakeVector` (`KismetMathLibrary.RandomFloatInRange` 10.0 50.0) (`KismetMathLibrary.RandomFloatInRange` 10.0 50.0) (`KismetMathLibrary.RandomFloatInRange` 10.0 50.0)))
  (set `self.HitBoneName` HitBoneName)
  (return))

(fn `UserConstructionScript`)